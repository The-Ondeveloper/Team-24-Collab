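; BP_PlayerCharacter is the player-controlled Character, handling movement, look and jump input through events.
; Move input drives AddMovementInput along forward and right vectors built from actor yaw only.
; Look input adds controller yaw scaled by LookSensitivity, while pitch is only inverted, as its sensitivity multiply is left unconnected.
; Jump input calls Jump, and BeginPlay, Possessed and the construction script are empty.
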(event Custom|OnMoveInput
  (params (Movement :type Vector%202D%20Structure))
  (bind _returnvalue (Transformation|GetActorRotation))
  (bind _yaw (Math|Rotator|BreakRotator _returnvalue))
  (bind _returnvalue_2 (Math|Rotator|MakeRotator 0.0 0.0 _yaw))
  (Pawn|Input|AddMovementInput (Math|Vector|GetRightVector _returnvalue_2) (.y Movement) false)
  (Pawn|Input|AddMovementInput (Math|Vector|GetForwardVector _returnvalue_2) (.x Movement) false))

(event Custom|OnLookInput
  (params (LookAxis :type Vector%202D%20Structure))
  (Pawn|Input|AddControllerYawInput (* (.x LookAxis) (Variables|Default|GetLookSensitivity)))
  (Pawn|Input|AddControllerPitchInput (* (.y LookAxis) -1.0)))

(event Custom|OnJumpInput
  (Character|Jump))

(event EventBeginPlay)

(event EventPossessed
  (params (NewController :type Controller%20Object%20Reference)))

(fn ConstructionScript)