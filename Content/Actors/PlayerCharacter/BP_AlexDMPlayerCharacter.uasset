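; Player character Blueprint that moves, jumps and looks through input events, with debug keys that apply damage or negative damage to itself.
; Movement follows the actor's yaw, and look sensitivity scales yaw only, while pitch is just inverted.
; On Health component death it asks GM_BaseGameMode to respawn the player, then re-initialises the HUD through the controller cached at BeginPlay.
; An AddForce event passes forces to CharacterMovement.
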(event OnDeath(Health)
  (bind _player_controller (Variables|Default|GetPlayer%20Controller))
  (bind _asgm_base_game_mode (Utilities|Casting|CastToGM_BaseGameMode (Game|GetGameMode)))
  (Class|BaseGameMode|RespawnPlayer _asgm_base_game_mode)
  (Default|InitialiseHUD (Variables|/Game/Input/PlayerController/PC_AlexDMPlayerController.PC_AlexDMPlayerController_C|GetPlayerHUDWidget _player_controller) (Variables|/Game/Input/PlayerController/PC_AlexDMPlayerController.PC_AlexDMPlayerController_C|GetControlledCharacter _player_controller)))

(event Custom|OnMoveInput
  (params (Movement :type Vector%202D%20Structure))
  (bind _returnvalue (Transformation|GetActorRotation))
  (bind _yaw (Math|Rotator|BreakRotator _returnvalue))
  (bind _returnvalue_2 (Math|Rotator|MakeRotator 0.0 0.0 _yaw))
  (Pawn|Input|AddMovementInput (Math|Vector|GetRightVector _returnvalue_2) (.y Movement) false)
  (Pawn|Input|AddMovementInput (Math|Vector|GetForwardVector _returnvalue_2) (.x Movement) false))

(event Custom|OnLookInput
  (params (LookAxis :type Vector%202D%20Structure))
  (Pawn|Input|AddControllerYawInput (* (.x LookAxis) (Variables|Default|GetLookSensitivity)))
  (Pawn|Input|AddControllerPitchInput (* (.y LookAxis) -1.0)))

(event Custom|OnJumpInput
  (Character|Jump))

(event EventAddForce
  (params (Force :type Vector :default "0, 0, 0"))
  (Physics|AddForce (Variables|Character|GetCharacterMovement) Force))

(event EventBeginPlay
  (bind _aspc_alex_dmplayer_controller (Utilities|Casting|CastToPC_AlexDMPlayerController (Pawn|GetController)))
  (Variables|Default|SetPlayer%20Controller _aspc_alex_dmplayer_controller))

(event EventPossessed
  (params (NewController :type Controller%20Object%20Reference)))

(event Input|KeyboardEvents|DebugKey1
  (params (Key :type Key%20Structure :default "None") (ActionValue :type Input%20Action%20Value%20Structure))
  ;[0.15 0.15 0.15 0.5] Debugging for Taking Damage and Applying Health
  (:Pressed
    (Game|Damage|ApplyDamage self 1e+01 0 0)))

(event Input|KeyboardEvents|DebugKey2
  (params (Key :type Key%20Structure :default "None") (ActionValue :type Input%20Action%20Value%20Structure))
  ;[0.15 0.15 0.15 0.5] Debugging for Taking Damage and Applying Health
  (:Pressed
    (Game|Damage|ApplyDamage self -1e+01 0 0)))

(fn ConstructionScript)