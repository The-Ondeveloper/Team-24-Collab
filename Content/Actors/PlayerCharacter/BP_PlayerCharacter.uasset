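; BP_PlayerCharacter is the player character, handling movement, jump and look input plus respawn on death.
; Movement follows actor yaw; look yaws the controller scaled by sensitivity, while pitch rotates the camera locally, unscaled and without any clamp here.
; On Health death it asks BaseGameMode to respawn, then resets the first Electric and Grapple abilities and adds their maximum energy.
; An AddForce event forwards external forces to CharacterMovement.
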(event OnDeath(Health)
  (bind _abilityelectric (Variables|Default|GetAbilityElectric))
  (bind _abilitygrapple (Variables|Default|GetAbilityGrapple))
  (bind _asbase_game_mode (Utilities|Casting|CastToBaseGameMode (Game|GetGameMode)))
  (Class|BaseGameMode|RespawnPlayer _asbase_game_mode)
  (Default|ResetAbility (Default|GetAbilityatIndex _abilityelectric))
  (Default|ModifyEnergy _abilityelectric (Variables|/Game/Actors/Components/C_CoreAbility.C_CoreAbility_C|GetMaxEnergy _abilityelectric))
  (Default|ResetAbility (Default|GetAbilityatIndex _abilitygrapple))
  (Default|ModifyEnergy _abilitygrapple (Variables|/Game/Actors/Components/C_CoreAbility.C_CoreAbility_C|GetMaxEnergy _abilitygrapple)))

(event Custom|OnMoveInput
  (params (Movement :type Vector%202D%20Structure))
  (bind _returnvalue (Transformation|GetActorRotation))
  (bind _yaw (Math|Rotator|BreakRotator _returnvalue))
  (bind _returnvalue_2 (Math|Rotator|MakeRotator 0.0 0.0 _yaw))
  (Pawn|Input|AddMovementInput (Math|Vector|GetRightVector _returnvalue_2) (.y Movement) false)
  (Pawn|Input|AddMovementInput (Math|Vector|GetForwardVector _returnvalue_2) (.x Movement) false))

(event Custom|OnLookInput
  (params (LookAxis :type Vector%202D%20Structure))
  (Pawn|Input|AddControllerYawInput (* (.x LookAxis) (Variables|Default|GetLookSensitivity)))
  (Transformation|AddLocalRotation (Variables|Default|GetCamera) (Math|Rotator|MakeRotator 0.0 (.y LookAxis) 0.0) false false))

(event Custom|OnJumpInput
  (Character|Jump))

(event EventBeginPlay)

(event EventAddForce
  (params (Force :type Vector :default "0, 0, 0"))
  (Physics|AddForce (Variables|Character|GetCharacterMovement) Force))

(event EventPossessed
  (params (NewController :type Controller%20Object%20Reference)))

(fn ConstructionScript)