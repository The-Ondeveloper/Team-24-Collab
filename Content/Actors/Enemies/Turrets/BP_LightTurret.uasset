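; Enemy turret that turns toward the player within its aggro sphere and can be temporarily stunned through OnPower.
; Tick lerps the pivot while a fire-rate timer runs a dot-product FOV check and forward line trace before applying damage, which also requires a valid fire sound.
; Dispatchers report detection, out-of-FOV, shot and lost-player events.
; A state widget initialised with the turret is turned to the player camera by a fast looping timer.
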(event OnComponentBeginOverlap(Sphere)
  (params (OverlappedComponent :type Primitive%20Component%20Object%20Reference) (OtherActor :type Actor%20Object%20Reference) (OtherComp :type Primitive%20Component%20Object%20Reference) (OtherBodyIndex :type Integer) (bFromSweep :type Boolean) (SweepResult :type Hit%20Result%20Structure%20%28by%20ref%29))
  ;[0.15 0.15 0.15 0.5] Detect Player
  (Variables|Default|SetPlayerInRange (== OtherActor (Variables|Default|GetPlayerRef)))
  (bind _returnvalue (Utilities|Time|SetTimerbyEvent (delegate Custom|FIre) (/ 1.0 (Variables|Default|GetFireRate)) true))
  (Variables|Default|SetFireTimer _returnvalue))

(event OnComponentEndOverlap(Sphere)
  (params (OverlappedComponent :type Primitive%20Component%20Object%20Reference) (OtherActor :type Actor%20Object%20Reference) (OtherComp :type Primitive%20Component%20Object%20Reference) (OtherBodyIndex :type Integer))
  ;[0.15 0.15 0.15 0.5] Player Left Range
  (bind _asbp_player_character (Utilities|Casting|CastToBP_PlayerCharacter OtherActor))
  (Utilities|IsValid _asbp_player_character
    (:Is%20Valid
      (Utilities|Time|PauseTimerbyHandle (Variables|Default|GetFireTimer))
      (Variables|Default|SetPlayerInRange false)
      (Default|CallEonLosePlayer self))))

(event Custom|FIre
  (bind _playerref (Variables|Default|GetPlayerRef))
  ;[0.15 0.15 0.15 0.5] Detect Player
  (Utilities|IsValid _playerref
    (:Is%20Valid
      (CallFunction|ShootatPlayer _playerref))))

(event Custom|ResumeFiring
  ;[0.15 0.15 0.15 0.5] Handle Stun
  (Variables|Default|SetCanFire true))

(event Custom|WidgetFacePlayer
  (Transformation|SetWorldRotation (Variables|Default|GetWidget) (Math|Rotator|FindLookatRotation (Transformation|GetWorldLocation (Variables|Default|GetWidget)) (Transformation|GetWorldLocation (Variables|/Game/Actors/PlayerCharacter/BP_PlayerCharacter.BP_PlayerCharacter_C|GetCamera (Variables|Default|GetPlayerRef)))) false false))

(event EventBeginPlay
  (bind _asbp_player_character (Utilities|Casting|CastToBP_PlayerCharacter (Game|GetPlayerCharacter 0)))
  (Variables|Default|SetPlayerRef _asbp_player_character)
  (bind _returnvalue (UserInterface|CreateWidget "/Game/UI/Turrets/WBP_TurretStateNotify.WBP_TurretStateNotify_C"))
  (bind _output_get (Variables|Default|SetTurretWidgetRef _returnvalue))
  (UserInterface|SetWidget (Variables|Default|GetWidget) _output_get)
  (Default|Initialise _output_get self)
  (bind _returnvalue_2 (Utilities|Time|SetTimerbyEvent (delegate Custom|WidgetFacePlayer) 0.001 true))
  (Variables|Default|SetWidgetLookAtPlayerTimer _returnvalue_2))

(event EventOnPower
  ;[0.15 0.15 0.15 0.5] Handle Stun
  (if (Variables|Default|GetCanFire)
    (Utilities|Time|SetTimerbyEvent (delegate Custom|ResumeFiring) (Variables|Default|GetStunTimer))
    (Variables|Default|SetCanFire false)))

(event EventTick
  (params (DeltaSeconds :type Float%20%28single-precision%29))
  (bind _pivotpoint (Variables|Default|GetPivotPoint))
  ;[0.15 0.15 0.15 0.5] Rotate Toward Player
  (if (and (Variables|Default|GetPlayerInRange) (Variables|Default|GetCanFire))
    (Transformation|SetWorldRotation _pivotpoint (Math|Rotator|Lerp(Rotator) (Transformation|GetWorldRotation _pivotpoint) (Math|Conversions|RotationFromXVector (- (Transformation|GetActorLocation (Variables|Default|GetPlayerRef)) (Transformation|GetWorldLocation (Variables|Default|GetPivotPoint)))) (* DeltaSeconds (Variables|Default|GetRotationSpeed)) true) false false)))

(fn ConstructionScript
  (Components|Sphere|SetSphereRadius (Variables|Default|GetSphere) (Variables|Default|GetAggroRange) true))

(fn ShootatPlayer
  (params (Player :type BP%20Player%20Character%20Object%20Reference%20%28by%20ref%29))
  (bind _firepoint (Variables|Default|GetFirePoint))
  (bind _firesound (Variables|Default|GetFireSound))
  (bind _returnvalue (Transformation|GetWorldLocation _firepoint))
  (if (Variables|Default|GetCanFire)
    (Default|CallEonPlayerDetected self)
    (bind _isinfov (CallFunction|IsPlayerinFOV Player (Variables|Default|GetFOV)))
    (if _isinfov
      (bind _outhit (Collision|LineTraceForObjects _returnvalue (+ _returnvalue (* (Math|Vector|GetForwardVector _firepoint) (Variables|Default|GetAggroRange))) (Utilities|Array|MakeArray "ObjectTypeQuery1" "ObjectTypeQuery3" "ObjectTypeQuery4" "ObjectTypeQuery2") false 0 "Persistent" true "(R=1.000000,G=0.000000,B=0.000000,A=1.000000)" "(R=0.000000,G=1.000000,B=0.000000,A=1.000000)" 1.0))
      (if (== (.HitActor (Collision|BreakHitResult _outhit)) Player)
        (Utilities|IsValid _firesound
          (:Is%20Valid
            (Default|CallEonShootatPlayer self)
            (Audio|PlaySoundatLocation _firesound (Transformation|GetActorLocation) "0, 0, 0" 1.0 1.0 0.0 0 0 0 0)
            (Game|Damage|ApplyDamage Player (Variables|Default|GetDamage) 0 self))))
      (else
        (Default|CallEonPlayerNotWithinFOV self)))))

(fn IsPlayerinFOV
  (params (Player :type BP%20Player%20Character%20Object%20Reference) (FOV :type Float%20%28double-precision%29))
  (return (> (Math|Vector|DotProduct (Math|Vector|GetForwardVector (Variables|Default|GetFirePoint)) (Math|Vector|Normalize (- (Transformation|GetActorLocation Player) (Transformation|GetWorldLocation (Variables|Default|GetFirePoint))))) (Math|Trig|Cos(Degrees) (/ FOV 2.0)))))

(fn GetMesh
  (return 0))

(fn ReturnGrappleAttachType
  (return (Variables|Default|GetAttachType)))