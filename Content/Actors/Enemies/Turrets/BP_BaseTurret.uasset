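; Base enemy turret that tracks and shoots the player inside an aggro sphere, and reports a grapple attach type.
; Overlap starts a looping fire timer, while Tick eases the pivot toward the player.
; Shots require an FOV dot-product check and a debug-drawn line trace hit, firing dispatchers along the way; damage only applies if FireSound is valid.
; OnPower stuns the turret, halting rotation and firing until a timer restores them.
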(event OnComponentBeginOverlap(Sphere)
  (params (OverlappedComponent :type Primitive%20Component%20Object%20Reference) (OtherActor :type Actor%20Object%20Reference) (OtherComp :type Primitive%20Component%20Object%20Reference) (OtherBodyIndex :type Integer) (bFromSweep :type Boolean) (SweepResult :type Hit%20Result%20Structure%20%28by%20ref%29))
  ;[0.15 0.15 0.15 0.5] Detect Player
  (bind _asbp_player_character (Utilities|Casting|CastToBP_PlayerCharacter OtherActor))
  (Utilities|IsValid _asbp_player_character
    (:Is%20Valid
      (Variables|Default|SetPlayerInRange true)
      (Variables|Default|SetPlayerRef _asbp_player_character)
      (bind _returnvalue (Utilities|Time|SetTimerbyEvent (delegate Custom|FIre) (/ 1.0 (Variables|Default|GetFireRate)) true))
      (Variables|Default|SetFireTimer _returnvalue))))

(event OnComponentEndOverlap(Sphere)
  (params (OverlappedComponent :type Primitive%20Component%20Object%20Reference) (OtherActor :type Actor%20Object%20Reference) (OtherComp :type Primitive%20Component%20Object%20Reference) (OtherBodyIndex :type Integer))
  ;[0.15 0.15 0.15 0.5] Player Left Range
  (bind _asbp_player_character (Utilities|Casting|CastToBP_PlayerCharacter OtherActor))
  (Utilities|IsValid _asbp_player_character
    (:Is%20Valid
      (Utilities|Time|PauseTimerbyHandle (Variables|Default|GetFireTimer))
      (Variables|Default|SetPlayerInRange false)
      (Default|CallEonLosePlayer self))))

(event Custom|FIre
  (bind _playerref (Variables|Default|GetPlayerRef))
  ;[0.15 0.15 0.15 0.5] Detect Player
  (Utilities|IsValid _playerref
    (:Is%20Valid
      (CallFunction|ShootatPlayer _playerref))))

(event Custom|ResumeFiring
  ;[0.15 0.15 0.15 0.5] Handle Stun
  (Variables|Default|SetCanFire true))

(event EventOnPower
  ;[0.15 0.15 0.15 0.5] Handle Stun
  (if (Variables|Default|GetCanFire)
    (Utilities|Time|SetTimerbyEvent (delegate Custom|ResumeFiring) (Variables|Default|GetStunTimer))
    (Variables|Default|SetCanFire false)))

(event EventTick
  (params (DeltaSeconds :type Float%20%28single-precision%29))
  (bind _pivotpoint (Variables|Default|GetPivotPoint))
  ;[0.15 0.15 0.15 0.5] Rotate Toward Player
  (if (and (Variables|Default|GetPlayerInRange) (Variables|Default|GetCanFire))
    (Transformation|SetWorldRotation _pivotpoint (Math|Rotator|Lerp(Rotator) (Transformation|GetWorldRotation _pivotpoint) (Math|Conversions|RotationFromXVector (- (Transformation|GetActorLocation (Variables|Default|GetPlayerRef)) (Transformation|GetWorldLocation (Variables|Default|GetPivotPoint)))) (* DeltaSeconds (Variables|Default|GetRotationSpeed)) true) false false)))

(fn ConstructionScript
  (Components|Sphere|SetSphereRadius (Variables|Default|GetSphere) (Variables|Default|GetAggroRange) true))

(fn ShootatPlayer
  (params (Player :type BP%20Player%20Character%20Object%20Reference%20%28by%20ref%29))
  (bind _firepoint (Variables|Default|GetFirePoint))
  (bind _firesound (Variables|Default|GetFireSound))
  (bind _returnvalue (Transformation|GetWorldLocation _firepoint))
  (if (Variables|Default|GetCanFire)
    (Default|CallEonPlayerDetected self)
    (bind _isinfov (CallFunction|IsPlayerinFOV Player (Variables|Default|GetFOV)))
    (if _isinfov
      (Default|CallEonPlayerWithinFOV self)
      (bind _outhit (Collision|LineTraceForObjects _returnvalue (+ _returnvalue (* (Math|Vector|GetForwardVector _firepoint) (Variables|Default|GetAggroRange))) (Utilities|Array|MakeArray "ObjectTypeQuery1" "ObjectTypeQuery3" "ObjectTypeQuery4" "ObjectTypeQuery2") false 0 "Persistent" true "(R=1.000000,G=0.000000,B=0.000000,A=1.000000)" "(R=0.000000,G=1.000000,B=0.000000,A=1.000000)" 1.0))
      (if (== (.HitActor (Collision|BreakHitResult _outhit)) Player)
        (Utilities|IsValid _firesound
          (:Is%20Valid
            (Default|CallEonShootatPlayer self)
            (Audio|PlaySoundatLocation _firesound (Transformation|GetActorLocation) "0, 0, 0" 1.0 1.0 0.0 0 0 0 0)
            (Game|Damage|ApplyDamage Player (Variables|Default|GetDamage) 0 self)))))))

(fn IsPlayerinFOV
  (params (Player :type BP%20Player%20Character%20Object%20Reference) (FOV :type Float%20%28double-precision%29))
  (return (> (Math|Vector|DotProduct (Math|Vector|GetForwardVector (Variables|Default|GetFirePoint)) (Math|Vector|Normalize (- (Transformation|GetActorLocation Player) (Transformation|GetWorldLocation (Variables|Default|GetFirePoint))))) (Math|Trig|Cos(Degrees) (/ FOV 2.0)))))

(fn GetMesh
  (return 0))

(fn ReturnGrappleAttachType
  (return (Variables|Default|GetAttachType)))