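; BP_Lvl1DoubleDoor is a triggered double door prop that slides open and closes itself after a delay.
; OnTrigger toggles the powered flag and calls DoorOpen, which activates the door and runs DoorEvent.
; DoorEvent plays a timeline that lerps both panels' relative locations if active and powered, otherwise reverses it.
; After DoorOpenTimer, OnTrigger clears both flags and reverses the timeline.
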(event Custom|DoorEvent
  (if (and (Variables|Default|GetDoorActive) (Variables|Default|GetDoorPowered))
    (bind _doorprogress (Timeline|Timeline Play)
      (:Update
        (Transformation|SetRelativeLocation (Variables|Default|GetDoorLeft) (Math|Vector|Lerp(Vector) (Variables|Default|GetLA) (Variables|Default|GetLB) _doorprogress) false false)
        (Transformation|SetRelativeLocation (Variables|Default|GetDoorRight) (Math|Vector|Lerp(Vector) (Variables|Default|GetRA) (Variables|Default|GetRB) _doorprogress) false false)))
    (else
      (Timeline|Timeline Reverse))))

(event EventOnTrigger
  (Variables|Default|SetDoorPowered (not (Variables|Default|GetDoorPowered)))
  (CallFunction|DoorOpen)
  (Utilities|FlowControl|Delay (Variables|Default|GetDoorOpenTimer))
  (Variables|Default|SetDoorActive false)
  (Variables|Default|SetDoorPowered false)
  (bind _doorprogress (Timeline|Timeline Reverse)
    (:Update
      (Transformation|SetRelativeLocation (Variables|Default|GetDoorLeft) (Math|Vector|Lerp(Vector) (Variables|Default|GetLA) (Variables|Default|GetLB) _doorprogress) false false)
      (Transformation|SetRelativeLocation (Variables|Default|GetDoorRight) (Math|Vector|Lerp(Vector) (Variables|Default|GetRA) (Variables|Default|GetRB) _doorprogress) false false))))

(fn ConstructionScript
  (|CallParentFunction))

(fn DoorOpen
  (if (Variables|Default|GetDoorActive)
    _
    (else
      _))
  (if (Variables|Default|GetDoorPowered)
    _
    (else
      _))
  (Variables|Default|SetDoorActive true)
  (CallFunction|DoorEvent))