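; Single sliding door prop that opens when enough power sources trigger it and closes when the count drops below its threshold.
; Trigger and untrigger events adjust a PowerSources counter, compare it to PowerThreshold, then play the open or close sound and animation.
; A Slide_Vertical timeline lerps the door between closed and open relative locations, reversing to close.
; The construction script places the door according to IsOpen.
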(event Custom|PlayAnimation
  (params (Play%20Forward :type Boolean))
  (if Play%20Forward
    (bind _floatlerp (Timeline|Slide_Vertical Play)
      (:Update
        (Transformation|SetRelativeLocation (Variables|Default|GetSlidingDoor) (Math|Vector|Lerp(Vector) (Variables|DoorData|GetClosedLocation) (Variables|DoorData|GetOpenLocation) _floatlerp) false false)))
    (else
      (Timeline|Slide_Vertical Reverse))))

(event EventOnUnTrigger
  (Math|Integer|DecrementInt (Variables|Default|GetPowerSources)
    (:%20%20
      (if (< (Variables|Default|GetPowerSources) (Variables|DoorData|GetPowerThreshold))
        (bind _output_get (Variables|DoorData|SetIsOpen false))
        (CallFunction|PlayAnimation _output_get)
        (Audio|PlaySoundatLocation (Variables|Sounds|GetDoorClose) (Transformation|GetActorLocation) "0, 0, 0" 1.0 1.0 0.0 0 0 0 0)))))

(event EventOnTrigger
  (Math|Integer|IncrementInt (Variables|Default|GetPowerSources)
    (:%20%20
      (if (>= (Variables|Default|GetPowerSources) (Variables|DoorData|GetPowerThreshold))
        (bind _output_get (Variables|DoorData|SetIsOpen true))
        (CallFunction|PlayAnimation _output_get)
        (Audio|PlaySoundatLocation (Variables|Sounds|GetDoorOpen) (Transformation|GetActorLocation) "0, 0, 0" 1.0 1.0 0.0 0 0 0 0)))))

(fn ConstructionScript
  (bind _slidingdoor (Variables|Default|GetSlidingDoor))
  (if (Variables|DoorData|GetIsOpen)
    (Transformation|SetRelativeLocation _slidingdoor (Variables|DoorData|GetOpenLocation) false false)
    (else
      (Transformation|SetRelativeLocation _slidingdoor (Variables|DoorData|GetClosedLocation) false false))))