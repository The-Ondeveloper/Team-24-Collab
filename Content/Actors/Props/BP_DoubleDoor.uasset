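; Double sliding door prop that extends a parent Blueprint with a second panel, SlidingDoorB.
; PlayAnimation plays or reverses the SlideHorizontal timeline, lerping both panels between their closed and open relative locations.
; The construction script calls the parent, then snaps the second panel to match IsOpen.
; Trigger and untrigger events only forward to the parent.
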(event EventBeginPlay)

(event Collision|EventActorBeginOverlap
  (params (OtherActor :type Actor%20Object%20Reference)))

(event EventTick
  (params (DeltaSeconds :type Float%20%28single-precision%29)))

(event EventOnTrigger
  (|CallParentFunction))

(event EventOnUnTrigger
  (|CallParentFunction))

(event EventPlayAnimation
  (params (Play%20Forward :type Boolean))
  (if Play%20Forward
    (bind _lerp (Timeline|Slide%20Horizontal Play)
      (:Update
        (Transformation|SetRelativeLocation (Variables|Default|GetSlidingDoor) (Math|Vector|Lerp(Vector) (Variables|Default|GetClosedLocation) (Variables|Default|GetOpenLocation) _lerp) false false)
        (Transformation|SetRelativeLocation (Variables|Default|GetSlidingDoorB) (Math|Vector|Lerp(Vector) (Variables|DoorData|GetClosedLocationB) (Variables|DoorData|GetOpenLocationB) _lerp) false false)))
    (else
      (Timeline|Slide%20Horizontal Reverse))))

(fn ConstructionScript
  (bind _slidingdoorb (Variables|Default|GetSlidingDoorB))
  (|CallParentFunction)
  (if (Variables|Default|GetIsOpen)
    (Transformation|SetRelativeLocation _slidingdoorb (Variables|DoorData|GetOpenLocationB) false false)
    (else
      (Transformation|SetRelativeLocation _slidingdoorb (Variables|DoorData|GetClosedLocationB) false false))))