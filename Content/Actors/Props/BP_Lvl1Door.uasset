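; BP_Lvl1Door is a door prop that slides open and closed as its powered state is toggled.
; OnTrigger flips DoorPowered, then DoorOpen sets DoorActive to true and calls DoorEvent.
; DoorEvent plays a Timeline when both flags are true and reverses it otherwise, lerping the Door's relative location between StartLocation and OffsetLocation.
; DoorOpen's branches on both flags are empty, so DoorPowered alone decides the direction on each trigger.
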(event Custom|DoorEvent
  (if (and (Variables|Default|GetDoorActive) (Variables|Default|GetDoorPowered))
    (bind _doorprogress (Timeline|Timeline Play)
      (:Update
        (Transformation|SetRelativeLocation (Variables|Default|GetDoor) (Math|Vector|Lerp(Vector) (Variables|Default|GetStart%20Location) (Variables|Default|GetOffset%20Location) _doorprogress) false false)))
    (else
      (Timeline|Timeline Reverse))))

(event EventBeginPlay)

(event Collision|EventActorBeginOverlap
  (params (OtherActor :type Actor%20Object%20Reference)))

(event EventTick
  (params (DeltaSeconds :type Float%20%28single-precision%29)))

(event EventOnTrigger
  (Variables|Default|SetDoorPowered (not (Variables|Default|GetDoorPowered)))
  (CallFunction|DoorOpen))

(fn ConstructionScript
  (|CallParentFunction))

(fn DoorOpen
  (if (Variables|Default|GetDoorActive)
    _
    (else
      _))
  (if (Variables|Default|GetDoorPowered)
    _
    (else
      _))
  (Variables|Default|SetDoorActive true)
  (CallFunction|DoorEvent))