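; BP_CubeRespawner is a prop that spawns an actor of a configurable class at its SpawnPoint and returns it there on demand.
; BeginPlay stores the spawned actor and binds to its damage event, so damage resets the cube, as does OnTrigger.
; Respawning reuses the same actor, moving it to the spawn point, zeroing its rotation and calling HaltMomentumMessage to stop its motion.
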(event Custom|Spawn%20Cube
  (bind _cuberef (Variables|Default|GetCubeRef))
  (Transformation|SetActorLocation _cuberef (Transformation|GetWorldLocation (Variables|Default|GetSpawnPoint)) false false)
  (Transformation|SetActorRotation _cuberef)
  (Class|IPhysicsActor|HaltMomentum(Message) _cuberef))

(event Custom|RespawnCube
  (params (DamagedActor :type Actor%20Object%20Reference) (Damage :type Float%20%28single-precision%29) (DamageType :type Damage%20Type%20Object%20Reference) (InstigatedBy :type Controller%20Object%20Reference) (DamageCauser :type Actor%20Object%20Reference))
  (CallFunction|SpawnCube))

(event EventBeginPlay
  (bind _returnvalue (Game|SpawnActorfromClass (Variables|SpawnerData|GetObjectToSpawn) (Math|Transform|MakeTransform (Transformation|GetWorldLocation (Variables|Default|GetSpawnPoint))) "AdjustIfPossibleButAlwaysSpawn" "MultiplyWithRoot" 0 0))
  (bind _output_get (Variables|Default|SetCubeRef _returnvalue))
  (EventDispatchers|BindEventtoOnTakeAnyDamage _output_get (EventDispatchers|CreateEvent :!event Custom|RespawnCube)))

(event Collision|EventActorBeginOverlap
  (params (OtherActor :type Actor%20Object%20Reference)))

(event EventTick
  (params (DeltaSeconds :type Float%20%28single-precision%29)))

(event EventOnTrigger
  (CallFunction|SpawnCube))

(fn ConstructionScript)