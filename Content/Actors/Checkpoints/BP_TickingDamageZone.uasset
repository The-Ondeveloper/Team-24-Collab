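; Checkpoint-derived zone that, once activated, repeatedly damages the actors overlapping its collider.
; CheckpointActivated starts a looping timer after a start delay, with a handle validity check to avoid creating a second one.
; Each tick of that timer calls DamageEntities, which applies the configured damage to every overlapped actor, with no filtering and no stop logic in this graph.
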(event Custom|DamageEntities
  (for _array_element (Variables|/Script/Team24Project.Collider|GetOverlappedActors (Variables|Default|GetCollider))
    (Game|Damage|ApplyDamage _array_element (Variables|Default|GetDamage) 0 0)))

(event EventCheckpointActivated
  (params (OverlappedActor :type Actor%20Object%20Reference))
  (if (not (Utilities|Time|IsValidTimerHandle (Variables|Default|GetDamageTimer)))
    (bind _returnvalue (Utilities|Time|SetTimerbyEvent (delegate Custom|DamageEntities) (Variables|Default|GetDamageDelay) true false (Variables|Default|GetStartDelay)))
    (Variables|Default|SetDamageTimer _returnvalue)))

(fn ConstructionScript
  (|CallParentFunction))