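; Grapple ability actor that pulls objects toward itself, riding attached to its owning actor and hidden until a hook lands.
; Activation sphere-traces along the player's control rotation and attaches the PullHook's end to the hit component.
; Holding applies distance-scaled, delta-time force to the hooked actor's root primitive and changes energy by a per-second cost.
; Cancelling, including on a failed trace or hold, hides the actor and resets the hook.
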(event EventBeginPlay
  (bind _owning_actor (Variables|Default|GetOwning%20Actor))
  (bind _returnvalue (Actor|GetComponentbyClass _owning_actor "/Script/Engine.SceneComponent"))
  (Rendering|SetActorHiddenInGame true)
  (|CallParentFunction)
  (Utilities|IsValid _returnvalue
    (:Is%20Valid
      (Transformation|AttachComponentToComponent _returnvalue "None" "SnapToTarget" "SnapToTarget" "KeepWorld" false))))

(event Collision|EventActorBeginOverlap
  (params (OtherActor :type Actor%20Object%20Reference))
  (|CallParentFunction OtherActor) ; This node is disabled and will not be called.\nDrag off pins to build functionality.
)

(event EventTick
  (params (DeltaSeconds :type Float%20%28single-precision%29))
  (|CallParentFunction DeltaSeconds) ; This node is disabled and will not be called.\nDrag off pins to build functionality.
)

(fn ConstructionScript
  (|CallParentFunction))

(fn ActivateAbility
  (params (Force%20Activation :type Boolean) (CurrentEnergy :type Float%20%28double-precision%29))
  (bind _returnvalue (Transformation|GetActorLocation))
  (bind _attributes (Variables|Default|GetAttributes))
  (bind (_range _abilityradius) (Utilities|Struct|BreakS_AbilityAttributes _attributes))
  (bind _output_get (LocalVariables|SetEnergy CurrentEnergy))
  (if (or Force%20Activation (CallFunction|CanUseAbilitywithEnergy _output_get))
    (bind (_outhit _returnvalue_2) (Collision|SphereTraceForObjects _returnvalue (+ _returnvalue (* (Math|Vector|GetForwardVector (Pawn|GetControlRotation (Game|GetPlayerController 0) :!class /Script/Engine.Controller)) _range)) _abilityradius (LocalVariables|GetObjectTypes) false 0 "None"))
    (if _returnvalue_2
      (Rendering|SetActorHiddenInGame false)
      (Class|CableComponent|SetAttachEndtoComponent (Variables|Default|GetPullHook) (.HitComponent (Collision|BreakHitResult _outhit)) "None")
      (Default|CallOnPrimaryUsed true)
      (return true (LocalVariables|GetEnergy))
      (else
        (CallFunction|CancelAbility (LocalVariables|GetEnergy))
        (Default|CallOnPrimaryUsed false)
        (return false (LocalVariables|GetEnergy))))))

(fn CancelAbility
  (params (Current%20Energy :type Float%20%28double-precision%29))
  (Rendering|SetActorHiddenInGame true)
  (Class|CableComponent|SetAttachEndtoComponent (Variables|Default|GetPullHook) (Variables|Default|GetDefaultSceneRoot) "None")
  (Default|CallOnPrimaryCancelled true)
  (return true Current%20Energy))

(fn HoldAbility
  (params (Current%20Energy :type Float%20%28double-precision%29))
  (bind _pullhook (Variables|Default|GetPullHook))
  (bind _pullhook_2 (Variables|Default|GetPullHook))
  (bind _returnvalue (Class|CableComponent|GetAttachedComponent _pullhook))
  (bind _returnvalue_2 (Class|CableComponent|GetAttachedActor _pullhook_2))
  (LocalVariables|SetEnergy Current%20Energy)
  (if (Math|Boolean|ANDBoolean (CallFunction|CanUseAbilitywithEnergy Current%20Energy) (Utilities|IsValid _returnvalue) (!= _returnvalue (Variables|Default|GetDefaultSceneRoot)))
    (bind _asprimitive_component (Utilities|Casting|CastToPrimitiveComponent (Variables|/Script/Engine.Actor|GetRootComponent _returnvalue_2))
      (:then
        (Physics|AddForce _asprimitive_component (* (* (Math|Vector|GetUnitDirection(Vector) (Transformation|GetActorLocation _returnvalue_2) (Transformation|GetActorLocation)) (* (+ (* (Math|Vector|Distance(Vector) (Transformation|GetActorLocation (Class|CableComponent|GetAttachedActor (Variables|Default|GetPullHook))) (Transformation|GetActorLocation)) 0.5) 1e+03) (Utilities|Struct|BreakS_AbilityAttributes (Variables|Default|GetAttributes)))) (Utilities|Time|GetWorldDeltaSeconds)) "None" false)
        (Default|CallOnPrimaryHeld true)
        (bind _new_energy (CallFunction|ChangeEnergy (LocalVariables|GetEnergy) (* (Utilities|Struct|BreakS_AbilityAttributes (Variables|Default|GetAttributes)) (Utilities|Time|GetWorldDeltaSeconds))))
        (return true _new_energy))
      (:CastFailed
        (CallFunction|CancelAbility (LocalVariables|GetEnergy))
        (Default|CallOnPrimaryHeld false)
        (return false (LocalVariables|GetEnergy))))
    (else
      (CallFunction|CancelAbility (LocalVariables|GetEnergy))
      (Default|CallOnPrimaryHeld false)
      (return false (LocalVariables|GetEnergy)))))