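; Grapple hook ability actor, mounted on the owner's ElecAttachPoint, that pulls the character toward grapple points or reels physics objects in.
; Activation sphere-traces along camera aim for I_GrappleInterface actors, whose attach type selects the pull behaviour.
; Looping timers animate the cable's fire and retract, pinning it to physics meshes with a local-space offset.
; Holding applies distance-scaled force and drains energy, cancelling when energy runs out or range is exceeded.
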(event EventBeginPlay
  (bind _owning_actor (Variables|Default|GetOwning%20Actor))
  (bind _elecattachpoint (Variables|/Game/Actors/PlayerCharacter/BP_PlayerCharacter.BP_PlayerCharacter_C|GetElecAttachPoint _owning_actor))
  (Rendering|SetActorHiddenInGame true)
  (|CallParentFunction)
  (Utilities|IsValid _elecattachpoint
    (:Is%20Valid
      (Transformation|AttachComponentToComponent _elecattachpoint "None" "SnapToTarget" "SnapToTarget" "KeepWorld" false))))

(event Collision|EventActorBeginOverlap
  (params (OtherActor :type Actor%20Object%20Reference))
  (|CallParentFunction OtherActor) ; This node is disabled and will not be called.\nDrag off pins to build functionality.
)

(event EventTick
  (params (DeltaSeconds :type Float%20%28single-precision%29))
  (|CallParentFunction DeltaSeconds) ; This node is disabled and will not be called.\nDrag off pins to build functionality.
)

(fn ConstructionScript
  (|CallParentFunction))

(fn ActivateAbility
  (params (Force%20Activation :type Boolean) (CurrentEnergy :type Float%20%28double-precision%29))
  (bind _owning_actor (Variables|Default|GetOwning%20Actor))
  (bind _attributes (Variables|Default|GetAttributes))
  (bind (_range _abilityradius) (Utilities|Struct|BreakS_AbilityAttributes _attributes))
  (bind _camera (Variables|/Game/Actors/PlayerCharacter/BP_PlayerCharacter.BP_PlayerCharacter_C|GetCamera _owning_actor))
  (CallFunction|ResetAbility)
  (bind _output_get (LocalVariables|SetEnergy CurrentEnergy))
  (if (CallFunction|CanUseAbilitywithEnergy _output_get)
    (bind _output_get_2 (LocalVariables|SetMaxReachPoint (+ (Transformation|GetWorldLocation _camera) (* (Math|Vector|GetForwardVector (Transformation|GetWorldRotation _camera)) _range))))
    (bind (_outhit _returnvalue) (Collision|SphereTraceForObjects (Transformation|GetActorLocation) _output_get_2 _abilityradius (LocalVariables|GetObjectTypes) false (Utilities|Array|MakeArray (Variables|Default|GetOwning%20Actor)) "ForOneFrame"))
    (if _returnvalue
      (if (Utilities|DoesObjectImplementInterface (.HitActor (Collision|BreakHitResult _outhit)) "/Game/Actors/Abilities/GrappleHook/I_GrappleInterface.I_GrappleInterface_C")
        (Variables|Grapple|SetImpactLocation (.ImpactPoint (Collision|BreakHitResult _outhit)))
        (Variables|Grapple|SetHitActor (.HitActor (Collision|BreakHitResult _outhit)))
        (bind _attach_type (Class|IGrappleInterface|ReturnGrappleAttachType(Message) (.HitActor (Collision|BreakHitResult _outhit))))
        (Variables|Grapple|SetCurrentAttach _attach_type)
        (Animation|TriggerFireAnimation)
        (Default|CallOnPrimaryUsed true)
        (return true (LocalVariables|GetEnergy))
        (else
          (Default|CallOnPrimaryUsed false)
          (Variables|Grapple|SetImpactLocation (.ImpactPoint (Collision|BreakHitResult _outhit)))))
      (else
        (Default|CallOnPrimaryUsed false)
        (Variables|Grapple|SetImpactLocation (LocalVariables|GetMaxReachPoint))))
    (Variables|Grapple|SetCurrentAttach "NewEnumerator2")
    (Animation|TriggerFireAnimation)
    (return false (LocalVariables|GetEnergy))
    (else
      (Default|CallOnPrimaryUsed false)
      (return false 0.0))))

(fn HoldAbility
  (params (Current%20Energy :type Float%20%28double-precision%29))
  (LocalVariables|SetEnergy Current%20Energy)
  (if (and (Variables|Animation|GetAnimFinished) (Utilities|IsValid (Class|CableComponent|GetAttachedComponent (Variables|Default|GetGrappleHook))))
    (if (Math|Boolean|ANDBoolean (CallFunction|CanUseAbilitywithEnergy (LocalVariables|GetEnergy)) (<= (Math|Vector|Distance(Vector) (Transformation|GetWorldLocation (Class|CableComponent|GetAttachedComponent (Variables|Default|GetGrappleHook))) (Transformation|GetActorLocation)) (* (Utilities|Struct|BreakS_AbilityAttributes (Variables|Default|GetAttributes)) 1.5)) true)
      (switch Utilities|FlowControl|Switch|SwitchonE_AttachType (Variables|Grapple|GetCurrentAttach)
        (:NewEnumerator0
          (Grapple|ReelTowardsPoint))
        (:NewEnumerator1
          (Grapple|ReelinObject)))
      (bind _new_energy (CallFunction|ChangeEnergy (LocalVariables|GetEnergy) (* (.EnergyCost (Utilities|Struct|BreakS_AbilityAttributes (Variables|Default|GetAttributes))) (Utilities|Time|GetWorldDeltaSeconds))))
      (Default|CallOnPrimaryHeld true)
      (return true _new_energy)
      (else
        (CallFunction|CancelAbility 0.0)
        (Default|CallOnPrimaryHeld false)
        (return false (LocalVariables|GetEnergy))))
    (else
      (Default|CallOnPrimaryHeld false)
      (return false (LocalVariables|GetEnergy)))))

(fn CancelAbility
  (params (Current%20Energy :type Float%20%28double-precision%29))
  (Animation|TriggerFailAnimation)
  (Variables|Grapple|SetCurrentAttach "NewEnumerator2")
  (Variables|Grapple|SetHitActor 0)
  (Default|CallOnPrimaryCancelled true)
  (return true Current%20Energy))

(fn TriggerFireAnimation
  (bind _impactpoint (Variables|Default|GetImpactPoint))
  (Utilities|Time|ClearandInvalidateTimerbyHandle (Variables|Animation|GetGrappleFailTimer))
  (Variables|Animation|SetAnimFinished false)
  (Rendering|SetActorHiddenInGame false)
  (Transformation|SetWorldLocation _impactpoint (Transformation|GetActorLocation) false false)
  (Class|CableComponent|SetAttachEndtoComponent (Variables|Default|GetGrappleHook) _impactpoint "None")
  (bind _returnvalue (Utilities|Time|SetTimerbyEvent (EventDispatchers|CreateEvent :!event FireAnim) 1e-06 true true))
  (Variables|Animation|SetGrappleFireTimer _returnvalue))

(fn FireAnim
  (bind _returnvalue (Utilities|Time|GetWorldDeltaSeconds))
  (bind _impactpoint (Variables|Default|GetImpactPoint))
  (bind _impactlocation (Variables|Grapple|GetImpactLocation))
  (bind _attributes (Variables|Default|GetAttributes))
  (bind _chargetime (Utilities|Struct|BreakS_AbilityAttributes _attributes))
  (bind _returnvalue_2 (Transformation|GetWorldLocation _impactpoint))
  (bind _returnvalue_3 (Math|Interpolation|VInterptoConstant _returnvalue_2 _impactlocation _returnvalue _chargetime))
  (Transformation|SetWorldLocation (Variables|Default|GetImpactPoint) _returnvalue_3 false false)
  (if (Utilities|Operators|EqualEqual _returnvalue_3 (Variables|Grapple|GetImpactLocation) 0.1)
    (Utilities|Time|ClearandInvalidateTimerbyHandle (Variables|Animation|GetGrappleFireTimer))
    (Variables|Animation|SetAnimFinished true)
    (switch Utilities|FlowControl|Switch|SwitchonE_AttachType (Variables|Grapple|GetCurrentAttach)
      (:NewEnumerator2
        (CallFunction|CancelAbility 0.0))
      (:NewEnumerator1
        (bind _staticmesh (Class|IGrappleInterface|GetMesh(Message) (Variables|Grapple|GetHitActor)))
        (Class|CableComponent|SetAttachEndtoComponent (Variables|Default|GetGrappleHook) _staticmesh "None")
        (Animation|SetGrappleOffset (- (Variables|Grapple|GetImpactLocation) (Transformation|GetWorldLocation _staticmesh)))))))

(fn ReelTowardsPoint
  (bind _attributes (Variables|Default|GetAttributes))
  (bind _speed (Utilities|Struct|BreakS_AbilityAttributes _attributes))
  (if (not (Grapple|IsGrappleatShortRange (Transformation|GetActorLocation) (Transformation|GetWorldLocation (Class|CableComponent|GetAttachedComponent (Variables|Default|GetGrappleHook))) 1e+02))
    (Physics|AddForce (Actor|GetComponentbyClass (Variables|Default|GetOwning%20Actor) "/Script/Engine.CharacterMovementComponent") (* (* (Math|Vector|Normalize (Math|Vector|GetUnitDirection(Vector) (Transformation|GetActorLocation) (Transformation|GetWorldLocation (Class|CableComponent|GetAttachedComponent (Variables|Default|GetGrappleHook))))) (+ (* (+ (Math|Float|Min(Float) (/ (Math|Vector|Distance(Vector) (Transformation|GetActorLocation) (Transformation|GetWorldLocation (Class|CableComponent|GetAttachedComponent (Variables|Default|GetGrappleHook)))) (Utilities|Struct|BreakS_AbilityAttributes (Variables|Default|GetAttributes))) 2.0) 1e+02) _speed) (/ _speed 2.5))) (Utilities|Time|GetWorldDeltaSeconds)))))

(fn ReelinObject
  (bind _grapplehook (Variables|Default|GetGrappleHook))
  (bind _grapplehook_2 (Variables|Default|GetGrappleHook))
  (bind _returnvalue (Class|CableComponent|GetAttachedActor _grapplehook))
  (bind _returnvalue_2 (Class|CableComponent|GetAttachedActor _grapplehook_2))
  (bind (_origin _boxextent) (Collision|GetActorBounds _returnvalue_2 false false))
  (if (and (Utilities|DoesObjectImplementInterface _returnvalue "/Game/Actors/Abilities/GrappleHook/I_GrappleInterface.I_GrappleInterface_C") (not (Grapple|IsGrappleatShortRange (Transformation|GetActorLocation) _origin (* (Math|Vector|VectorLength _boxextent) 1.21))))
    (bind _staticmesh (Class|IGrappleInterface|GetMesh(Message) _returnvalue))
    (Class|PrimitiveComponent|AddForceatLocationLocal _staticmesh (Math|Vector|RotateVector (* (* (Math|Vector|GetUnitDirection(Vector) (CallFunction|GetActorCentreWorldLocation _returnvalue) (Transformation|GetWorldLocation (Variables|Default|GetDefaultSceneRoot))) (* (+ (* (Math|Vector|Distance(Vector) (Transformation|GetActorLocation (Class|CableComponent|GetAttachedActor (Variables|Default|GetGrappleHook))) (Transformation|GetWorldLocation (Variables|Default|GetDefaultSceneRoot))) 0.5) 1e+03) (Utilities|Struct|BreakS_AbilityAttributes (Variables|Default|GetAttributes)))) (Utilities|Time|GetWorldDeltaSeconds)) (Class|KismetMathLibrary|NegateRotator (Transformation|GetWorldRotation _staticmesh))) (Variables|/Script/CableComponent.CableComponent|GetEndLocation (Variables|Default|GetGrappleHook)) "None")))

(fn TriggerFailAnimation
  (bind _impactpoint (Variables|Default|GetImpactPoint))
  (Utilities|Time|ClearandInvalidateTimerbyHandle (Variables|Animation|GetGrappleFireTimer))
  (Variables|Animation|SetAnimFinished false)
  (switch Utilities|FlowControl|Switch|SwitchonE_AttachType (Variables|Grapple|GetCurrentAttach)
    (:NewEnumerator2
      _)
    (:NewEnumerator0
      (Transformation|SetWorldLocation _impactpoint (Variables|Grapple|GetImpactLocation) false false))
    (:NewEnumerator1
      (Transformation|SetWorldLocation _impactpoint (+ (Transformation|GetActorLocation (Variables|Grapple|GetHitActor)) (Variables|Animation|GetGrapple%20Offset)) false false)))
  (Class|CableComponent|SetAttachEndtoComponent (Variables|Default|GetGrappleHook) (Variables|Default|GetImpactPoint) "None")
  (Variables|/Script/CableComponent.CableComponent|SetEndLocation (Variables|Default|GetGrappleHook) "0, 0, 0")
  (bind _returnvalue (Utilities|Time|SetTimerbyEvent (EventDispatchers|CreateEvent :!event FailAnim) 1e-06 true true))
  (Variables|Animation|SetGrappleFailTimer _returnvalue))

(fn FailAnim
  (bind _returnvalue (Transformation|GetActorLocation))
  (bind _returnvalue_2 (Utilities|Time|GetWorldDeltaSeconds))
  (bind _impactpoint (Variables|Default|GetImpactPoint))
  (bind _attributes (Variables|Default|GetAttributes))
  (bind _chargetime (Utilities|Struct|BreakS_AbilityAttributes _attributes))
  (bind _returnvalue_3 (Transformation|GetWorldLocation _impactpoint))
  (bind _returnvalue_4 (Math|Interpolation|VInterptoConstant _returnvalue_3 _returnvalue _returnvalue_2 _chargetime))
  (Transformation|SetWorldLocation (Variables|Default|GetImpactPoint) _returnvalue_4 false false)
  (if (Utilities|Operators|EqualEqual _returnvalue_4 _returnvalue 0.1)
    (Utilities|Time|ClearandInvalidateTimerbyHandle (Variables|Animation|GetGrappleFailTimer))
    (Rendering|SetActorHiddenInGame true)
    (Variables|Animation|SetAnimFinished true)))

(fn GetGrappleAnimSpeed
  (params (Current :type Vector) (To :type Vector) (Start :type Vector))
  (LocalVariables|SetA Current)
  (LocalVariables|SetB To)
  (LocalVariables|SetC Start)
  (return (* (Variables|Animation|GetAnimSpeed) (/ (Math|Vector|Distance(Vector) (LocalVariables|GetA) (LocalVariables|GetB)) (Math|Vector|Distance(Vector) (LocalVariables|GetB) (LocalVariables|GetC))))))

(fn IsGrappleatShortRange
  (params (Vector%20A :type Vector) (Vector%20B :type Vector) (Tolerance :type Float%20%28double-precision%29))
  (return (< (Math|Vector|Distance(Vector) Vector%20A Vector%20B) Tolerance)))

(fn SetGrappleOffset
  (params (Offset :type Vector))
  (Variables|Animation|SetGrapple%20Offset Offset)
  (bind _hitactor (Variables|Grapple|GetHitActor)
    (:then
      (bind _staticmesh (Class|IGrappleInterface|GetMesh(Message) _hitactor))
      (Variables|/Script/CableComponent.CableComponent|SetEndLocation (Variables|Default|GetGrappleHook) (/ (Math|Vector|RotateVector (Variables|Animation|GetGrapple%20Offset) (Class|KismetMathLibrary|NegateRotator (Transformation|GetWorldRotation _staticmesh))) (Transformation|GetWorldScale _staticmesh))))
    (:else)))

(fn ResetAbility
  (Variables|/Script/CableComponent.CableComponent|SetEndLocation (Variables|Default|GetGrappleHook) "0, 0, 0")
  (Utilities|Time|ClearandInvalidateTimerbyHandle (Variables|Animation|GetGrappleFireTimer))
  (Utilities|Time|ClearandInvalidateTimerbyHandle (Variables|Animation|GetGrappleFailTimer))
  (Variables|Grapple|SetCurrentAttach "NewEnumerator2")
  (Variables|Grapple|SetHitActor 0)
  (Rendering|SetActorHiddenInGame false)
  (Class|CableComponent|SetAttachEndtoComponent (Variables|Default|GetGrappleHook) 0 "None")
  (Variables|Animation|SetAnimFinished false)
  (Rendering|SetActorHiddenInGame true))