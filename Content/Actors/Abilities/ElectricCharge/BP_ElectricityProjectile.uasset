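; Electricity projectile for the electric charge ability, which charges up while attached and then launches to power objects it hits.
; Tick grows the Niagara core radius from start to target values over a set grow duration.
; FireProjectile detaches it and sets projectile movement velocity along the passed camera rotation.
; On sphere hit it sends a power message to Powerable actors, plays an electric hit sound and destroys itself.
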(event OnComponentHit(Sphere)
  (params (HitComponent :type Primitive%20Component%20Object%20Reference) (OtherActor :type Actor%20Object%20Reference) (OtherComp :type Primitive%20Component%20Object%20Reference) (NormalImpulse :type Vector :default "0, 0, 0") (Hit :type Hit%20Result%20Structure%20%28by%20ref%29))
  (if (Utilities|DoesObjectImplementInterface OtherActor "/Script/Team24Project.Powerable")
    (Class|Powerable|OnPower(Message) OtherActor))
  (Audio|PlaySoundatLocation "/Game/Audio/SoundEffects/MetaSounds/MS_ElectricHit.MS_ElectricHit" (Transformation|GetActorLocation) "0, 0, 0" 1.0 1.0 0.0 "/Game/Attenuation_Default.Attenuation_Default" 0 0 0)
  (Actor|DestroyActor))

(event Custom|FireProjectile
  (params (CameraRotation :type Rotator))
  (Transformation|DetachFromActor "KeepWorld" "KeepWorld" "KeepWorld")
  (Components|Activation|Activate (Variables|Default|GetProjectileMovement) false)
  ;[0.15 0.15 0.15 0.5] Placeholder (change to keep reference to camera)
  (Variables|/Script/Engine.MovementComponent|SetVelocity (Variables|Default|GetProjectileMovement) (* (Math|Rotator|GetRotationXVector CameraRotation) (Variables|Default|GetProjectileSpeed))))

(event EventBeginPlay
  (Variables|Default|SetCurrentGrowTime 0.0))

(event Collision|EventActorBeginOverlap
  (params (OtherActor :type Actor%20Object%20Reference)))

(event EventTick
  (params (DeltaSeconds :type Float%20%28single-precision%29))
  (bind _niagara (Variables|Default|GetNiagara))
  (bind _output_get (Variables|Default|SetCurrentGrowTime (Math|Float|Clamp(Float) (+ (Variables|Default|GetCurrentGrowTime) DeltaSeconds) 0.0 (Variables|Default|GetGrowDuration))))
  (Niagara|SetNiagaraVariable(Float) _niagara "CoreRadiusMin" (Math|Float|Lerp (Variables|Default|GetStartCoreRadiusMin) (Variables|Default|GetTargetCoreRadiusMin) (/ _output_get (Variables|Default|GetGrowDuration))))
  (Niagara|SetNiagaraVariable(Float) _niagara "CoreRadiusMax" (Math|Float|Lerp (Variables|Default|GetStartCoreRadiusMax) (Variables|Default|GetTargetCoreRadiusMax) (/ _output_get (Variables|Default|GetGrowDuration)))))

(fn ConstructionScript)