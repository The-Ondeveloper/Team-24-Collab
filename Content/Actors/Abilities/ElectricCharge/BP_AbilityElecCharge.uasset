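; Charged electricity ability that gives the player an electricity projectile to hold and then fire.
; Activation spawns BP_ElectricityProjectile, stores it and attaches it to the player character's projectile attach point before calling the parent ability logic.
; Release fires the stored projectile along the owning actor's camera rotation and clears the reference, while cancel destroys it.
; Each override passes the parent's success and energy results back to the caller.
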(event EventBeginPlay
  (|CallParentFunction) ; This node is disabled and will not be called.\nDrag off pins to build functionality.
)

(event Collision|EventActorBeginOverlap
  (params (OtherActor :type Actor%20Object%20Reference))
  (|CallParentFunction OtherActor) ; This node is disabled and will not be called.\nDrag off pins to build functionality.
)

(fn ConstructionScript
  (|CallParentFunction))

(fn ActivateAbility
  (params (Force%20Activation :type Boolean) (CurrentEnergy :type Float%20%28double-precision%29))
  ;[0.15 0.15 0.15 0.5] Using spawn electricity projectile and set ref. Then attach actor to player projectile attach point. The using parent activate ability and set is charging to true, charge to 1and charge timer to 0
  (bind _asbp_player_character (Utilities|Casting|CastToBP_PlayerCharacter (Pawn|GetControlledPawn (Game|GetPlayerController 0))))
  (bind _returnvalue (Game|SpawnActorfromClass "/Game/Actors/Abilities/ElectricCharge/BP_ElectricityProjectile.BP_ElectricityProjectile_C" (Math|Transform|MakeTransform (Transformation|GetWorldLocation (Variables|Default|GetDefaultSceneRoot)) "0, 0, 0" "1.000000,1.000000,1.000000") "AlwaysSpawn" "MultiplyWithRoot" 0 0))
  (Development|PrintString "Hello")
  (bind _output_get (Variables|Default|SetProjectile _returnvalue))
  (Transformation|AttachComponentToComponent _output_get (Variables|/Game/Actors/PlayerCharacter/BP_PlayerCharacter.BP_PlayerCharacter_C|GetProjectileAttachPoint _asbp_player_character) "None" "KeepRelative" "KeepRelative" "KeepRelative" true)
  (bind (_wassuccessful _remainingenergy) (|CallParentFunction Force%20Activation CurrentEnergy))
  (return _wassuccessful _remainingenergy))

(fn ReleaseAbility
  (params (Current%20Energy :type Float%20%28double-precision%29))
  ;[0.15 0.15 0.15 0.5] If release function called, set is charging to false, and set current charge back to 1, then firing projectile
  (bind (_successful _newenergy) (|CallParentFunction Current%20Energy))
  (Default|FireProjectile (Variables|Default|GetProjectile) (Transformation|GetWorldRotation (Variables|/Game/Actors/PlayerCharacter/BP_PlayerCharacter.BP_PlayerCharacter_C|GetCamera (Variables|Default|GetOwning%20Actor))))
  (Variables|Default|SetProjectile 0)
  (return _successful _newenergy))

(fn CancelAbility
  (params (Current%20Energy :type Float%20%28double-precision%29))
  (bind (_wascancelled _newenergy) (|CallParentFunction Current%20Energy))
  (Development|PrintString "CANCEL")
  (Actor|DestroyActor (Variables|Default|GetProjectile))
  (return _wascancelled _newenergy))