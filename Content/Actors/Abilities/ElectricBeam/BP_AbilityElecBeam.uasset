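; Electric beam ability that lets the player power objects in front of them while firing.
; Activation spawns a BP_ElecBeamEffect attached to the player character's ElecAttachPoint, and release destroys it, both calling the parent ability logic.
; Holding runs a short forward line trace from that point and sends OnPowerMessage to hit actors implementing Powerable.
; The hold's parent call is unconnected, and the owner lookup through player controller 0 is marked temporary.
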(event EventBeginPlay
  (|CallParentFunction) ; This node is disabled and will not be called.\nDrag off pins to build functionality.
)

(event Collision|EventActorBeginOverlap
  (params (OtherActor :type Actor%20Object%20Reference))
  (|CallParentFunction OtherActor) ; This node is disabled and will not be called.\nDrag off pins to build functionality.
)

(fn ConstructionScript
  (|CallParentFunction))

(fn ActivateAbility
  (params (Force%20Activation :type Boolean) (CurrentEnergy :type Float%20%28double-precision%29))
  ;[1 0.06301 0 0.502] Set owner on spawn instead
  (bind _asbp_player_character (Utilities|Casting|CastToBP_PlayerCharacter (Pawn|GetControlledPawn (Game|GetPlayerController 0))))
  (Variables|Default|SetbIsFiring true)
  (bind _returnvalue (Game|SpawnActorfromClass "/Game/Actors/Abilities/ElectricBeam/BP_ElecBeamEffect.BP_ElecBeamEffect_C" (Math|Transform|MakeTransform (Transformation|GetActorLocation _asbp_player_character) "0, 0, 0" "1.000000,1.000000,1.000000") "Undefined" "MultiplyWithRoot" 0 (Math|Vector|MakeVector 1e+02 0.0 0.0) 0))
  (bind _output_get (Variables|Default|SetBeam _returnvalue))
  (Transformation|AttachComponentToComponent _output_get (Variables|/Game/Actors/PlayerCharacter/BP_PlayerCharacter.BP_PlayerCharacter_C|GetElecAttachPoint _asbp_player_character) "None" "KeepRelative" "KeepRelative" "KeepRelative" true)
  (bind (_wassuccessful _remainingenergy) (|CallParentFunction Force%20Activation CurrentEnergy))
  (return _wassuccessful _remainingenergy))

(fn ReleaseAbility
  (params (Current%20Energy :type Float%20%28double-precision%29))
  (Variables|Default|SetbIsFiring false)
  (bind (_successful _newenergy) (|CallParentFunction Current%20Energy))
  (Actor|DestroyActor (Variables|Default|GetBeam))
  (return _successful _newenergy))

(fn HoldAbility
  (params (Current%20Energy :type Float%20%28double-precision%29))
  ;[1 0.06301 0 0.502] 100% cannot do this in final version - create owner variable for abilities
  (bind _asbp_player_character (Utilities|Casting|CastToBP_PlayerCharacter (Pawn|GetControlledPawn (Game|GetPlayerController 0))))
  ;[0.9655 1 0 0.5] Sphere trace might be better
  (bind _outhit (Collision|LineTraceByChannel (Transformation|GetWorldLocation (Variables|/Game/Actors/PlayerCharacter/BP_PlayerCharacter.BP_PlayerCharacter_C|GetElecAttachPoint _asbp_player_character)) (Math|Transform|TransformLocation (Transformation|GetWorldTransform (Variables|/Game/Actors/PlayerCharacter/BP_PlayerCharacter.BP_PlayerCharacter_C|GetElecAttachPoint _asbp_player_character)) "100.000000,0.000000,0.000000") "TraceTypeQuery1" false 0 "ForOneFrame"))
  (if (Utilities|DoesObjectImplementInterface (.hitactor _outhit) "/Script/Team24Project.Powerable")
    (Class|Powerable|OnPower(Message) (.hitactor _outhit))))