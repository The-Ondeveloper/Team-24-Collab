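; Grapple-in ability actor that pulls its owning character toward an aimed surface while held, at an energy cost.
; Activation sphere-traces along the control rotation, moves ImpactPoint to the hit and attaches the GrappleHook cable end there.
; Holding adds movement force blending hook direction with aim, scaled by distance and speed, and applies energy cost over time.
; Cancelling hides the actor and returns the cable end to its root.
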(event EventBeginPlay
  (bind _owning_actor (Variables|Default|GetOwning%20Actor))
  (bind _returnvalue (Actor|GetComponentbyClass _owning_actor "/Script/Engine.SceneComponent"))
  (Rendering|SetActorHiddenInGame true)
  (|CallParentFunction)
  (Utilities|IsValid _returnvalue
    (:Is%20Valid
      (Transformation|AttachComponentToComponent _returnvalue "None" "SnapToTarget" "SnapToTarget" "KeepWorld" false))))

(event Collision|EventActorBeginOverlap
  (params (OtherActor :type Actor%20Object%20Reference))
  (|CallParentFunction OtherActor) ; This node is disabled and will not be called.\nDrag off pins to build functionality.
)

(event EventTick
  (params (DeltaSeconds :type Float%20%28single-precision%29))
  (|CallParentFunction DeltaSeconds) ; This node is disabled and will not be called.\nDrag off pins to build functionality.
)

(fn ConstructionScript
  (|CallParentFunction))

(fn ActivateAbility
  (params (Force%20Activation :type Boolean) (CurrentEnergy :type Float%20%28double-precision%29))
  (bind _returnvalue (Transformation|GetActorLocation))
  (bind _attributes (Variables|Default|GetAttributes))
  (bind _impactpoint (Variables|Default|GetImpactPoint))
  (bind (_range _abilityradius) (Utilities|Struct|BreakS_AbilityAttributes _attributes))
  (LocalVariables|SetEnergy CurrentEnergy)
  (if (or Force%20Activation (CallFunction|CanUseAbilitywithEnergy CurrentEnergy))
    (bind (_outhit _returnvalue_2) (Collision|SphereTraceForObjects _returnvalue (+ _returnvalue (* (Math|Vector|GetForwardVector (Pawn|GetControlRotation (Game|GetPlayerController 0) :!class /Script/Engine.Controller)) _range)) _abilityradius (LocalVariables|GetObjectTypes) false 0 "ForOneFrame"))
    (if _returnvalue_2
      (Rendering|SetActorHiddenInGame false)
      (Transformation|SetWorldLocation _impactpoint (.ImpactPoint (Collision|BreakHitResult _outhit)) false false)
      (Class|CableComponent|SetAttachEndtoComponent (Variables|Default|GetGrappleHook) _impactpoint "None")
      (Default|CallOnPrimaryUsed true)
      (return true (LocalVariables|GetEnergy))
      (else
        (Default|CallOnPrimaryUsed false)
        (bind _newenergy (CallFunction|CancelAbility (LocalVariables|GetEnergy)))
        (return false _newenergy)))))

(fn HoldAbility
  (params (Current%20Energy :type Float%20%28double-precision%29))
  (bind _grapplehook (Variables|Default|GetGrappleHook))
  (bind _returnvalue (Class|CableComponent|GetAttachedComponent _grapplehook))
  (LocalVariables|SetEnergy Current%20Energy)
  (if (Math|Boolean|ANDBoolean (Utilities|IsValid _returnvalue) (!= _returnvalue (Variables|Default|GetDefaultSceneRoot)) (CallFunction|CanUseAbilitywithEnergy (LocalVariables|GetEnergy)))
    (Physics|AddForce (Actor|GetComponentbyClass (Variables|Default|GetOwning%20Actor) "/Script/Engine.CharacterMovementComponent") (* (* (Math|Vector|Normalize (+ (Math|Vector|GetUnitDirection(Vector) (Transformation|GetActorLocation) (Transformation|GetWorldLocation (Class|CableComponent|GetAttachedComponent (Variables|Default|GetGrappleHook)))) (* (Math|Vector|GetForwardVector (Pawn|GetControlRotation (Game|GetPlayerController 0) :!class /Script/Engine.Controller)) 0.7))) (* (+ (* (Math|Vector|Distance(Vector) (Transformation|GetActorLocation) (Transformation|GetWorldLocation (Class|CableComponent|GetAttachedComponent (Variables|Default|GetGrappleHook)))) 0.5) 1e+03) (Utilities|Struct|BreakS_AbilityAttributes (Variables|Default|GetAttributes)))) (Utilities|Time|GetWorldDeltaSeconds)))
    (bind _new_energy (CallFunction|ChangeEnergy (LocalVariables|GetEnergy) (* (Utilities|Struct|BreakS_AbilityAttributes (Variables|Default|GetAttributes)) (Utilities|Time|GetWorldDeltaSeconds))))
    (Default|CallOnPrimaryHeld true)
    (return true _new_energy)
    (else
      (bind _newenergy (CallFunction|CancelAbility (LocalVariables|GetEnergy)))
      (Default|CallOnPrimaryHeld false)
      (return false _newenergy))))

(fn CancelAbility
  (params (Current%20Energy :type Float%20%28double-precision%29))
  (Rendering|SetActorHiddenInGame true)
  (Class|CableComponent|SetAttachEndtoComponent (Variables|Default|GetGrappleHook) (Variables|Default|GetDefaultSceneRoot) "None")
  (Default|CallOnPrimaryCancelled true)
  (return true Current%20Energy))