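; Base physics prop actor that can be pushed by forces, picked up and queried for a grapple attach type.
; The construction script applies a configurable mesh and optional material to the Cube component, which receives all forces.
; Pickup refuses too-heavy objects, otherwise toggles gravity, simulation and collision while held.
; Hits above a velocity tolerance play a random impact sound, throttled by a short delay; Interact is an empty stub.
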(event OnComponentHit(Cube)
  (params (HitComponent :type Primitive%20Component%20Object%20Reference) (OtherActor :type Actor%20Object%20Reference) (OtherComp :type Primitive%20Component%20Object%20Reference) (NormalImpulse :type Vector :default "0, 0, 0") (Hit :type Hit%20Result%20Structure%20%28by%20ref%29))
  (if (and (Variables|Default|GetPlaySound) (Utilities|Operators|NotEqual(!=) :A (Transformation|GetVelocity) :ErrorTolerance 75.0))
    (Variables|Default|SetPlaySound false)
    (Audio|PlaySoundatLocation (.OutItem (Utilities|Array|Random (Variables|Default|GetHitSounds))) (Transformation|GetActorLocation) "0, 0, 0" 1.0 1.0 0.0 0 0 0 0)
    (Utilities|FlowControl|RetriggerableDelay 0.25)
    (Variables|Default|SetPlaySound true)))

(event EventBeginPlay)

(event Collision|EventActorBeginOverlap
  (params (OtherActor :type Actor%20Object%20Reference)))

(event EventTick
  (params (DeltaSeconds :type Float%20%28single-precision%29)))

(event EventAddForce
  (params (Force :type Vector :default "0, 0, 0"))
  (Physics|AddForce (Variables|Default|GetCube) Force "None" false))

(event EventAddForceatPoint
  (params (Force :type Vector :default "0, 0, 0") (Location :type Vector :default "0, 0, 0"))
  (Class|PrimitiveComponent|AddForceatLocation (Variables|Default|GetCube) Force Location "None"))

(event EventInteract)

(fn ConstructionScript
  (Components|StaticMesh|SetStaticMesh (Variables|Default|GetCube) (Variables|Default|GetMesh))
  (bind _override_material (Variables|Default|GetOverride%20Material)
    (:then
      (Rendering|Material|SetMaterial (Variables|Default|GetCube) 0 _override_material))
    (:else)))

(fn GetMesh
  (return (Variables|Default|GetCube)))

(fn Pickup
  (params (IsHeld :type Boolean))
  (bind _returnvalue (not IsHeld))
  (bind _cube (Variables|Default|GetCube))
  (bind _cube_2 (Variables|Default|GetCube))
  (if (Variables|Default|GetTooHeavy)
    (return false)
    (else
      (Physics|SetEnableGravity _cube _returnvalue)
      ;[0.15 0.15 0.15 0.5] Delete if Pickup becomes physics based
      (Physics|SetSimulatePhysics _cube _returnvalue)
      (if IsHeld
        (Collision|SetCollisionEnabled _cube_2 "NoCollision")
        (Development|PrintString "DisableCollision")
        (else
          (Collision|SetCollisionEnabled _cube_2 "QueryAndPhysics")))
      (return true))))

(fn ReturnGrappleAttachType
  (return "NewEnumerator1"))