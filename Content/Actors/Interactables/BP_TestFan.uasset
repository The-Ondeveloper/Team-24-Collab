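; Switchable fan that pushes physics actors along its up axis, inside a wind box sized from FanRange at construction.
; An I_PhysicsActor entering the box starts a next-tick loop that sends overlapping actors force scaled inversely with distance while powered and occupied.
; A line trace back toward the fan skips blocked actors.
; OnTrigger toggles power and the Timeline-driven blade spin, but does not restart the wind loop.
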(event OnActorEnterOverlap(WindArea)
  (params (OverlappedActor :type Actor%20Object%20Reference))
  (if (Utilities|DoesObjectImplementInterface OverlappedActor "/Game/Actors/Interactables/I_PhysicsActor.I_PhysicsActor_C")
    (CallFunction|StartWind)))

(event OnActorExitOverlap(WindArea)
  (params (OverlappedActor :type Actor%20Object%20Reference))
  (Variables|Default|SetbFanActive (Utilities|Array|IsNotEmpty (Collision|GetOverlappingActors (Variables|Default|GetWindArea) 0 :!class /Script/Engine.PrimitiveComponent))))

(event Custom|ApplyWind
  (if (and (Variables|Default|GetbFanActive) (Variables|FanData|GetIsPoweredOn))
    (for _array_element (Collision|GetOverlappingActors (Variables|Default|GetWindArea) 0 :!class /Script/Engine.PrimitiveComponent)
      (if (not (CallFunction|IsBlocked _array_element))
        (Class|IPhysicsActor|AddForce(Message) _array_element (* (* (Math|Vector|GetUpVector (Transformation|GetWorldRotation (Variables|Default|GetFanMesh))) (* (/ (Variables|FanData|GetFanRange) (Math|Vector|Distance(Vector) (Transformation|GetActorLocation _array_element) (Transformation|GetWorldLocation (Variables|Default|GetFanMesh)))) (Variables|FanData|GetFanPower))) (Utilities|Time|GetWorldDeltaSeconds)))))
    (Utilities|FlowControl|DelayUntilNextTick)
    (CallFunction|ApplyWind)))

(event Custom|Fan%20Spin
  (if (Variables|FanData|GetIsPoweredOn)
    (bind _newtrack_0 (Timeline|Timeline_0 Play)
      (:Update
        (Transformation|SetRelativeRotation (Variables|Default|GetFanMesh) (Math|Rotator|Lerp(Rotator) (Variables|Default|GetA) (Variables|Default|GetB) _newtrack_0) true false)))
    (else
      (Timeline|Timeline_0 Stop))))

(event EventBeginPlay
  (Utilities|FlowControl|DelayUntilNextTick)
  (Collision|SetCollisionEnabled (Variables|Default|GetWindArea) "QueryOnly")
  (CallFunction|FanSpin))

(event Collision|EventActorBeginOverlap
  (params (OtherActor :type Actor%20Object%20Reference)))

(event EventTick
  (params (DeltaSeconds :type Float%20%28single-precision%29)))

(event EventOnTrigger
  (Variables|FanData|SetIsPoweredOn (not (Variables|FanData|GetIsPoweredOn)))
  (CallFunction|FanSpin))

(fn ConstructionScript
  (bind _windarea (Variables|Default|GetWindArea))
  (bind _windarea_2 (Variables|Default|GetWindArea))
  (bind _windarea_3 (Variables|Default|GetWindArea))
  (bind _relativelocation (Variables|/Script/Engine.SceneComponent|GetRelativeLocation _windarea))
  (bind _boxextent (Variables|/Script/Engine.BoxComponent|GetBoxExtent _windarea_2))
  (bind _relativescale3d (Variables|/Script/Engine.SceneComponent|GetRelativeScale3D _windarea_3))
  (Transformation|SetRelativeLocation _windarea (Math|Vector|MakeVector (.x _relativelocation) (.y _relativelocation) (+ (.z _relativelocation) (/ (Variables|FanData|GetFanRange) 1.0))) false false)
  (Components|Box|SetBoxExtent _windarea_2 (Math|Vector|MakeVector (.x _boxextent) (.y _boxextent) (Variables|FanData|GetFanRange)) true)
  (Transformation|SetRelativeScale3D _windarea_3 (Math|Vector|MakeVector (.x _relativescale3d) (.y _relativescale3d) 1.0)))

(fn StartWind
  (if (Variables|Default|GetbFanActive)
    _
    (else
      _))
  (if (Variables|FanData|GetIsPoweredOn)
    _
    (else
      _))
  (Variables|Default|SetbFanActive true)
  (CallFunction|ApplyWind))

(fn IsBlocked
  (params (Actor :type Actor%20Object%20Reference))
  (bind _output_get (Variables|Default|SetActor Actor))
  (bind (_outhit _returnvalue) (Collision|LineTraceForObjects (CallFunction|GetActorCentreWorldLocation _output_get) (+ (+ (CallFunction|GetActorCentreWorldLocation _output_get) (* (* (Variables|FanData|GetFanRange) 2.0) (Math|Vector|NegateVector (Math|Vector|GetUpVector (Transformation|GetActorRotation))))) 1e+01) (LocalVariables|GetObjectTypes) false (Utilities|Array|MakeArray (Variables|Default|GetActor)) "ForOneFrame" false))
  (if (== (Variables|Default|GetFanMesh) (.HitComponent (Collision|BreakHitResult _outhit)))
    (return false)
    (else
      (return _returnvalue))))