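; BP_GrappleHookSurface is an interactable actor that serves as a configurable surface for the grapple hook.
; The construction script applies the chosen Mesh to BaseMesh and, if a valid OverrideMaterial is set, replaces the first material slot.
; Two query functions expose BaseMesh and a fixed grapple attach type, the enum's NewEnumerator0.
; It has no runtime event logic of its own.
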(event EventBeginPlay)

(event Collision|EventActorBeginOverlap
  (params (OtherActor :type Actor%20Object%20Reference)))

(event EventTick
  (params (DeltaSeconds :type Float%20%28single-precision%29)))

(fn ConstructionScript
  (Components|StaticMesh|SetStaticMesh (Variables|Default|GetBaseMesh) (Variables|GrappleSurface|GetMesh))
  (bind _overridematerial (Variables|GrappleSurface|GetOverrideMaterial)
    (:then
      (Rendering|Material|SetMaterial (Variables|Default|GetBaseMesh) 0 _overridematerial))
    (:else)))

(fn GetMesh
  (return (Variables|Default|GetBaseMesh)))

(fn ReturnGrappleAttachType
  (return "NewEnumerator0"))