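; Interactable button that adds its stored energy to the player's Electric or Grapple ability, selected by AbilityToCharge.
; On interact it passes EnergyLevel to that ability's ModifyEnergy, then optionally drains its own energy, clamped between zero and its starting amount.
; When regeneration is enabled, a looping timer restores one point per tick, pausing once full and unpausing after a draining use.
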(event Custom|RegenCharge
  ;[0.15 0.15 0.15 0.5] Handle Energy Recharging
  (if (Variables|Default|GetDoesDebugEnergy)
    (Development|PrintString (Utilities|String|ToString(Float) (Variables|Default|GetEnergyLevel))))
  (if (>= (Variables|Default|GetEnergyLevel) (Variables|Default|GetStartingEnergy))
    (Utilities|Time|PauseTimerbyHandle (Variables|Default|GetRegenTimer))
    (else
      (Variables|Default|SetEnergyLevel (+ (Variables|Default|GetEnergyLevel) 1.0)))))

(event EventInteract
  ;[0.15 0.15 0.15 0.5] Add Energy to selected ability
  (bind _asbp_player_character (Utilities|Casting|CastToBP_PlayerCharacter (Game|Player|GetPlayerPawn 0)))
  (switch Utilities|FlowControl|Switch|SwitchonAbilityTypes (Variables|Default|GetAbilityToCharge)
    (:NewEnumerator0
      (Default|ModifyEnergy (Variables|/Game/Actors/PlayerCharacter/BP_PlayerCharacter.BP_PlayerCharacter_C|GetAbilityElectric _asbp_player_character) (Variables|Default|GetEnergyLevel)))
    (:NewEnumerator1
      (Default|ModifyEnergy (Variables|/Game/Actors/PlayerCharacter/BP_PlayerCharacter.BP_PlayerCharacter_C|GetAbilityGrapple _asbp_player_character) (Variables|Default|GetEnergyLevel))))
  (if (Variables|Default|GetDoesLoseEnergy)
    (Variables|Default|SetEnergyLevel (Math|Float|Clamp(Float) (- (Variables|Default|GetEnergyLevel) (Variables|Default|GetEnergyLostOnUse)) 0.0 (Variables|Default|GetStartingEnergy)))
    (Utilities|Time|UnpauseTimerbyHandle (Variables|Default|GetRegenTimer))))

(event EventBeginPlay
  ;[0.15 0.15 0.15 0.5] Create Timer
  (Variables|Default|SetStartingEnergy (Variables|Default|GetEnergyLevel))
  (if (Variables|Default|GetDoesRegainEnergy)
    (bind _returnvalue (Utilities|Time|SetTimerbyEvent (delegate Custom|RegenCharge) (Variables|Default|GetEnergyRegenRate) true))
    (Variables|Default|SetRegenTimer _returnvalue)))

(fn ConstructionScript
  (|CallParentFunction))