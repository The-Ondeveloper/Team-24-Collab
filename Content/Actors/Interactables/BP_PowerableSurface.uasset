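; BP_PowerableSurface is an interactable surface that relays power events to the actors in TriggerTargets.
; OnPower flips IsPowered and sends each target a trigger or untrigger message to match.
; With TogglesBetweenTriggers set, the state persists, swaps the cube's material and, if initially powered, fires at BeginPlay.
; Otherwise IsPowered resets after each call, so every power event sends a trigger.
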(event Custom|SetPoweredMaterial
  (bind _cube (Variables|Default|GetCube))
  (if (Variables|Default|GetIsPowered)
    (Rendering|Material|SetMaterial _cube 0 "/Game/Materials/Instances/M_PoweredSurface.M_PoweredSurface")
    (else
      (Rendering|Material|SetMaterial _cube 0 "/Game/Materials/Instances/M_Powerable.M_Powerable"))))

(event EventBeginPlay
  (if (Variables|Default|GetTogglesBetweenTriggers)
    (CallFunction|SetPoweredMaterial)
    (if (Variables|Default|GetIsPowered)
      (Variables|Default|SetIsPowered false)
      (CallFunction|OnPower))
    (else
      (Variables|Default|SetIsPowered false))))

(event Collision|EventActorBeginOverlap
  (params (OtherActor :type Actor%20Object%20Reference)))

(event EventTick
  (params (DeltaSeconds :type Float%20%28single-precision%29)))

(event EventOnPower
  (Variables|Default|SetIsPowered (not (Variables|Default|GetIsPowered)))
  (for _array_element (Variables|Default|GetTriggerTargets)
    (if (Variables|Default|GetIsPowered)
      (Class|Triggerable|OnTrigger(Message) _array_element)
      (else
        (Class|Triggerable|OnUnTrigger(Message) _array_element))))
  (if (Variables|Default|GetTogglesBetweenTriggers)
    (CallFunction|SetPoweredMaterial)
    (else
      (Variables|Default|SetIsPowered false))))

(fn ConstructionScript)