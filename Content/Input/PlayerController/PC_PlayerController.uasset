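; Player controller that routes Enhanced Input to the possessed BP_PlayerCharacter for movement, grapple, electric charge and interaction.
; Ability inputs forward press phases to ability components and set ABP_PlayerArms animation flags; electric release fires only when the animation reports ready.
; A control-rotation line trace tracks the closest Interactable, which Interact messages and picks up if it is a physics actor.
; It also creates the HUD, starts a looping look-at timer and toggles the pause menu.
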(event Input|EnhancedActionEvents|EnhancedInputActionIA_Interact
  (params (ActionValue :type Boolean) (ElapsedSeconds :type Float%20%28double-precision%29) (TriggeredSeconds :type Float%20%28double-precision%29) (InputAction :type Input%20Action%20Object%20Reference :default "/Game/Input/InputAssets/IA_Interact.IA_Interact"))
  (bind _closestintreractable (Variables|Default|GetClosestIntreractable))
  (bind _controlledcharacter (Variables|Default|GetControlledCharacter))
  (bind _pickup_ability (Variables|/Game/Actors/PlayerCharacter/BP_PlayerCharacter.BP_PlayerCharacter_C|GetPickup_Ability _controlledcharacter))
  (:Started
    (if (Default|GetHasItem _pickup_ability)
      (Default|DropItem _pickup_ability)
      (elif (Variables|Default|GetHasNearbyInteractable)
        (Utilities|IsValid _closestintreractable
          (:Is%20Valid
            (Development|PrintString (Utilities|GetDisplayName _closestintreractable))
            (if (Utilities|DoesObjectImplementInterface _closestintreractable "/Script/Team24Project.Interactable")
              (Class|Interactable|Interact(Message) _closestintreractable)
              (if (Utilities|DoesObjectImplementInterface (Variables|Default|GetClosestIntreractable) "/Game/Actors/Interactables/I_PhysicsActor.I_PhysicsActor_C")
                (Default|PickupItem (Variables|/Game/Actors/PlayerCharacter/BP_PlayerCharacter.BP_PlayerCharacter_C|GetPickup_Ability (Variables|Default|GetControlledCharacter)) (Variables|Default|GetClosestIntreractable))
                (Development|PrintString "Picked Up Item")))))))))

(event Input|EnhancedActionEvents|EnhancedInputActionIA_Jump
  (params (ActionValue :type Boolean) (ElapsedSeconds :type Float%20%28double-precision%29) (TriggeredSeconds :type Float%20%28double-precision%29) (InputAction :type Input%20Action%20Object%20Reference :default "/Game/Input/InputAssets/IA_Jump.IA_Jump"))
  (:Started
    (Default|OnJumpInput (Variables|Default|GetControlledCharacter))))

(event Input|EnhancedActionEvents|EnhancedInputActionIA_Move
  (params (ActionValue :type Vector%202D%20Structure) (ElapsedSeconds :type Float%20%28double-precision%29) (TriggeredSeconds :type Float%20%28double-precision%29) (InputAction :type Input%20Action%20Object%20Reference :default "/Game/Input/InputAssets/IA_Move.IA_Move"))
  (bind _armsanim (Variables|Default|GetArmsAnim))
  (:Triggered
    (Default|OnMoveInput (Variables|Default|GetControlledCharacter) ActionValue))
  (:Started
    (Variables|/Game/Actors/PlayerCharacter/ABP_PlayerArms.ABP_PlayerArms_C|SetIsWalking _armsanim true))
  (:Completed
    (Variables|/Game/Actors/PlayerCharacter/ABP_PlayerArms.ABP_PlayerArms_C|SetIsWalking _armsanim false)))

(event Input|EnhancedActionEvents|EnhancedInputActionIA_Look
  (params (ActionValue :type Vector%202D%20Structure) (ElapsedSeconds :type Float%20%28double-precision%29) (TriggeredSeconds :type Float%20%28double-precision%29) (InputAction :type Input%20Action%20Object%20Reference :default "/Game/Input/InputAssets/IA_Look.IA_Look"))
  (Default|OnLookInput (Variables|Default|GetControlledCharacter) ActionValue))

(event Input|EnhancedActionEvents|EnhancedInputActionIA_ElectricCharge
  (params (ActionValue :type Boolean) (ElapsedSeconds :type Float%20%28double-precision%29) (TriggeredSeconds :type Float%20%28double-precision%29) (InputAction :type Input%20Action%20Object%20Reference :default "/Game/Input/InputAssets/IA_ElectricCharge.IA_ElectricCharge"))
  (bind _controlledcharacter (Variables|Default|GetControlledCharacter))
  (bind _armsanim (Variables|Default|GetArmsAnim))
  (bind _abilityelectric (Variables|/Game/Actors/PlayerCharacter/BP_PlayerCharacter.BP_PlayerCharacter_C|GetAbilityElectric _controlledcharacter))
  (:Triggered
    (Default|UseAbilityatIndex _abilityelectric 0 "Triggered" false))
  (:Started
    (Variables|/Game/Actors/PlayerCharacter/ABP_PlayerArms.ABP_PlayerArms_C|SetElecAnimTime _armsanim 0.0)
    (Variables|/Game/Actors/PlayerCharacter/ABP_PlayerArms.ABP_PlayerArms_C|SetIsElecHeld _armsanim true)
    (Default|UseAbilityatIndex _abilityelectric 0 "Started" false))
  (:Completed
    (Variables|/Game/Actors/PlayerCharacter/ABP_PlayerArms.ABP_PlayerArms_C|SetIsElecHeld _armsanim false)
    (if (Variables|/Game/Actors/PlayerCharacter/ABP_PlayerArms.ABP_PlayerArms_C|GetIsElecReadyToFire _armsanim)
      (Default|UseAbilityatIndex _abilityelectric 0 "Completed" false)
      (else
        (Default|UseAbilityatIndex _abilityelectric 0 "Canceled" false)))))

(event Input|EnhancedActionEvents|EnhancedInputActionIA_GrappleHook
  (params (ActionValue :type Boolean) (ElapsedSeconds :type Float%20%28double-precision%29) (TriggeredSeconds :type Float%20%28double-precision%29) (InputAction :type Input%20Action%20Object%20Reference :default "/Game/Input/InputAssets/IA_GrappleHook.IA_GrappleHook"))
  (bind _armsanim (Variables|Default|GetArmsAnim))
  (bind _controlledcharacter (Variables|Default|GetControlledCharacter))
  (bind _abilitygrapple (Variables|/Game/Actors/PlayerCharacter/BP_PlayerCharacter.BP_PlayerCharacter_C|GetAbilityGrapple _controlledcharacter))
  (:Triggered
    (Default|UseAbilityatIndex _abilitygrapple 0 "Triggered" false))
  (:Started
    (Variables|/Game/Actors/PlayerCharacter/ABP_PlayerArms.ABP_PlayerArms_C|SetGrappleAnimTime _armsanim 0.0)
    (Variables|/Game/Actors/PlayerCharacter/ABP_PlayerArms.ABP_PlayerArms_C|SetIsGrappleHeld _armsanim true)
    (Default|UseAbilityatIndex _abilitygrapple 0 "Started" false))
  (:Completed
    (Variables|/Game/Actors/PlayerCharacter/ABP_PlayerArms.ABP_PlayerArms_C|SetIsGrappleHeld _armsanim false)
    (Default|UseAbilityatIndex _abilitygrapple 0 "Canceled" false)))

(event Input|EnhancedActionEvents|EnhancedInputActionIA_Pause
  (params (ActionValue :type Boolean) (ElapsedSeconds :type Float%20%28double-precision%29) (TriggeredSeconds :type Float%20%28double-precision%29) (InputAction :type Input%20Action%20Object%20Reference :default "/Game/Input/InputAssets/IA_Pause.IA_Pause"))
  (bind _self self)
  (:Started
    (if (not (Variables|Default|GetPauseMenuOpen))
      (Variables|Default|SetPauseMenuOpen true)
      (bind _returnvalue (UserInterface|CreateWidget "/Game/UI/Menus/WBP_PauseMenu.WBP_PauseMenu_C" _self))
      (bind _output_get (Variables|Default|SetPauseMenuWidget _returnvalue))
      (UserInterface|Viewport|AddtoViewport _output_get 0)
      (Default|InitialisePauseMenu _returnvalue _self)
      (else
        (Variables|Default|SetPauseMenuOpen false)
        (Widget|RemovefromParent (Variables|Default|GetPauseMenuWidget))
        (Game|SetGamePaused false)
        (Input|SetInputModeGameOnly _self false)
        (Variables|Default|SetbShowMouseCursor false)))))

(event EventCheckpointSet
  (Default|CallEonCheckPointSet))

(event EventBeginPlay
  (if (Pawn|IsLocalController)
    (bind _returnvalue (Utilities|Time|SetTimerbyEvent (EventDispatchers|CreateEvent :!event CheckforInteractables) 0.1 true true))
    (Variables|Default|SetLookAtTimer _returnvalue)
    (CallFunction|InitialisePlayerHUD)))

(event EventPossess
  (params (PossessedPawn :type Pawn%20Object%20Reference))
  (bind _asbp_player_character (Utilities|Casting|CastToBP_PlayerCharacter PossessedPawn))
  (bind _output_get (Variables|Default|SetControlledCharacter _asbp_player_character))
  (Input|AddMappingContext (PlayerController|LocalPlayerSubsystems|GetEnhancedInputLocalPlayerSubsystem) "/Game/Input/InputAssets/IMC_DefaultInput.IMC_DefaultInput" 0 "(bIgnoreAllPressedKeysUntilRelease=True,bForceImmediately=False,bNotifyUserSettings=False)")
  (bind _asabp_player_arms (Utilities|Casting|CastToABP_PlayerArms (Components|SkeletalMesh|GetAnimInstance (Variables|/Game/Actors/PlayerCharacter/BP_PlayerCharacter.BP_PlayerCharacter_C|GetArmsRig _output_get))))
  (Variables|Default|SetArmsAnim _asabp_player_arms))

(fn ConstructionScript)

(fn AddNewInteractable
  (params (Actor :type Actor%20Object%20Reference%20%28by%20ref%29))
  (bind _returnvalue (Game|GetPlayerCharacter 0))
  (bind _returnvalue_2 (Transformation|GetActorLocation _returnvalue))
  (Utilities|IsValid (Variables|Default|GetClosestIntreractable)
    (:Is%20Valid
      (if (< (Math|Vector|Distance(Vector) (Transformation|GetActorLocation Actor) _returnvalue_2) (Math|Vector|Distance(Vector) _returnvalue_2 (Transformation|GetActorLocation (Variables|Default|GetClosestIntreractable))))
        (Variables|Default|SetClosestIntreractable Actor)
        (else
          (return))))
    (:Is%20Not%20Valid
      (Variables|Default|SetClosestIntreractable Actor)))
  (Variables|Default|SetHasNearbyInteractable true))

(fn RemoveInteractable
  (params (Actor :type Actor%20Object%20Reference%20%28by%20ref%29))
  (if (== Actor (Variables|Default|GetClosestIntreractable))
    (Variables|Default|SetHasNearbyInteractable (not (== Actor (Variables|Default|GetClosestIntreractable))))
    (Variables|Default|SetClosestIntreractable 0)))

(fn CheckforInteractables
  (bind _controlledcharacter (Variables|Default|GetControlledCharacter))
  (bind _returnvalue (Transformation|GetActorLocation _controlledcharacter))
  (bind (_outhit _returnvalue_2) (Collision|LineTraceForObjects _returnvalue (+ _returnvalue (* (Math|Vector|GetForwardVector (Pawn|GetControlRotation :!class /Script/Engine.Controller)) 5e+02)) (LocalVariables|GetObjectTypes) false (Utilities|Array|MakeArray (Variables|Default|GetControlledCharacter)) "None"))
  (if (and _returnvalue_2 (Utilities|DoesObjectImplementInterface (.HitActor (Collision|BreakHitResult _outhit)) "/Script/Team24Project.Interactable"))
    (if (!= (.HitActor (Collision|BreakHitResult _outhit)) (Variables|Default|GetClosestIntreractable))
      (CallFunction|AddNewInteractable (.HitActor (Collision|BreakHitResult _outhit))))
    (else
      (bind _closestintreractable (Variables|Default|GetClosestIntreractable)
        (:then
          (CallFunction|RemoveInteractable _closestintreractable))
        (:else)))))

(fn InitialisePlayerHUD
  ;[0.15 0.15 0.15 0.5] Creates Player HUD and sets ref, then calls initialise event to then add to player screen
  (bind _returnvalue (UserInterface|CreateWidget "/Game/UI/PlayerHUD/WBP_PlayerHUD.WBP_PlayerHUD_C" self))
  (bind _output_get (Variables|Default|SetPlayerHUDWidget _returnvalue))
  (Default|InitialiseHUD _output_get (Variables|Default|GetControlledCharacter) self)
  (UserInterface|Viewport|AddtoPlayerScreen _output_get))