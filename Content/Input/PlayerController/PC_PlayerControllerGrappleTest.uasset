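; Player controller for the grapple test character that routes Enhanced Input to the possessed pawn.
; On possess it caches the character and adds the default input mapping context, with debug prints.
; Move, look and jump go to character input handlers.
; Ability inputs call UseAbilityAtIndex on the grapple and electric abilities with forced activation; mouse clicks forward started, triggered and completed phases to two electric slots.
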(event Input|EnhancedActionEvents|EnhancedInputActionIA_AbilityPrimary
  (params (ActionValue :type Boolean) (ElapsedSeconds :type Float%20%28double-precision%29) (TriggeredSeconds :type Float%20%28double-precision%29) (InputAction :type Input%20Action%20Object%20Reference :default "/Game/Input/InputAssets/IA_AbilityPrimary.IA_AbilityPrimary"))
  (:Started
    (Default|UseAbilityatIndex (Variables|/Game/Actors/PlayerCharacter/BP_PlayerCharacter_GrappleTest.BP_PlayerCharacter_GrappleTest_C|GetGrapple%20Ability (Variables|Default|GetControlledCharacter)) 0 "Started" true)))

(event Input|EnhancedActionEvents|EnhancedInputActionIA_Jump
  (params (ActionValue :type Boolean) (ElapsedSeconds :type Float%20%28double-precision%29) (TriggeredSeconds :type Float%20%28double-precision%29) (InputAction :type Input%20Action%20Object%20Reference :default "/Game/Input/InputAssets/IA_Jump.IA_Jump"))
  (:Started
    (Default|OnJumpInput (Variables|Default|GetControlledCharacter))))

(event Input|EnhancedActionEvents|EnhancedInputActionIA_Move
  (params (ActionValue :type Vector%202D%20Structure) (ElapsedSeconds :type Float%20%28double-precision%29) (TriggeredSeconds :type Float%20%28double-precision%29) (InputAction :type Input%20Action%20Object%20Reference :default "/Game/Input/InputAssets/IA_Move.IA_Move"))
  (Default|OnMoveInput (Variables|Default|GetControlledCharacter) ActionValue))

(event Input|EnhancedActionEvents|EnhancedInputActionIA_Look
  (params (ActionValue :type Vector%202D%20Structure) (ElapsedSeconds :type Float%20%28double-precision%29) (TriggeredSeconds :type Float%20%28double-precision%29) (InputAction :type Input%20Action%20Object%20Reference :default "/Game/Input/InputAssets/IA_Look.IA_Look"))
  (Default|OnLookInput (Variables|Default|GetControlledCharacter) ActionValue))

(event Input|EnhancedActionEvents|EnhancedInputActionIA_AbilitySecondary
  (params (ActionValue :type Boolean) (ElapsedSeconds :type Float%20%28double-precision%29) (TriggeredSeconds :type Float%20%28double-precision%29) (InputAction :type Input%20Action%20Object%20Reference :default "/Game/Input/InputAssets/IA_AbilitySecondary.IA_AbilitySecondary"))
  (Default|UseAbilityatIndex (Variables|/Game/Actors/PlayerCharacter/BP_PlayerCharacter_GrappleTest.BP_PlayerCharacter_GrappleTest_C|GetGrapple%20Ability (Variables|Default|GetControlledCharacter)) 0 "Triggered" true))

(event Input|EnhancedActionEvents|EnhancedInputActionIA_LeftClick
  (params (ActionValue :type Boolean) (ElapsedSeconds :type Float%20%28double-precision%29) (TriggeredSeconds :type Float%20%28double-precision%29) (InputAction :type Input%20Action%20Object%20Reference :default "/Game/Input/InputAssets/IA_LeftClick.IA_LeftClick"))
  (bind _controlledcharacter (Variables|Default|GetControlledCharacter))
  (bind _electric_ability (Variables|/Game/Actors/PlayerCharacter/BP_PlayerCharacter_GrappleTest.BP_PlayerCharacter_GrappleTest_C|GetElectric%20Ability _controlledcharacter))
  (:Triggered
    (Default|UseAbilityatIndex _electric_ability 0 "Triggered" true))
  (:Started
    (Default|UseAbilityatIndex _electric_ability 0 "Started" true))
  (:Completed
    (Default|UseAbilityatIndex _electric_ability 0 "Completed" true)))

(event Input|EnhancedActionEvents|EnhancedInputActionIA_RightClick
  (params (ActionValue :type Boolean) (ElapsedSeconds :type Float%20%28double-precision%29) (TriggeredSeconds :type Float%20%28double-precision%29) (InputAction :type Input%20Action%20Object%20Reference :default "/Game/Input/InputAssets/IA_RightClick.IA_RightClick"))
  (bind _controlledcharacter (Variables|Default|GetControlledCharacter))
  (bind _electric_ability (Variables|/Game/Actors/PlayerCharacter/BP_PlayerCharacter_GrappleTest.BP_PlayerCharacter_GrappleTest_C|GetElectric%20Ability _controlledcharacter))
  (:Triggered
    (Default|UseAbilityatIndex _electric_ability 1 "Triggered" true))
  (:Started
    (Default|UseAbilityatIndex _electric_ability 1 "Started" true))
  (:Completed
    (Default|UseAbilityatIndex _electric_ability 1 "Completed" true)))

(event EventBeginPlay
  (Development|PrintString "PC begin play")
  (if (Pawn|IsLocalController)
    (Development|PrintString "true")))

(event EventPossess
  (params (PossessedPawn :type Pawn%20Object%20Reference))
  (bind _asbp_player_character_grapple_test (Utilities|Casting|CastToBP_PlayerCharacter_GrappleTest PossessedPawn)
    (:then
      (Variables|Default|SetControlledCharacter _asbp_player_character_grapple_test)
      (Development|PrintString "Pawn possessed")
      (Input|AddMappingContext (PlayerController|LocalPlayerSubsystems|GetEnhancedInputLocalPlayerSubsystem) "/Game/Input/InputAssets/IMC_DefaultInput.IMC_DefaultInput" 0 "(bIgnoreAllPressedKeysUntilRelease=True,bForceImmediately=False,bNotifyUserSettings=False)")
      (Development|PrintString "Input mapping context added"))
    (:CastFailed
      (Development|PrintString "Possess failed"))))

(fn ConstructionScript)