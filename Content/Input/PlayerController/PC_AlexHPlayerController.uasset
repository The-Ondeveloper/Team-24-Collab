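; Player controller that routes Enhanced Input to the possessed BP_PlayerCharacter and handles interaction with nearby objects.
; On possess it caches the character and adds the default mapping context, then forwards move, jump and look input to it.
; AddNewInteractable keeps only the closer candidate by distance at registration time, and RemoveInteractable clears it without a fallback.
; The interact action messages that stored actor through the Interactable interface.
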(event Input|EnhancedActionEvents|EnhancedInputActionIA_Interact
  (params (ActionValue :type Boolean) (ElapsedSeconds :type Float%20%28double-precision%29) (TriggeredSeconds :type Float%20%28double-precision%29) (InputAction :type Input%20Action%20Object%20Reference :default "/Game/Input/InputAssets/IA_Interact.IA_Interact"))
  (bind _closestintreractable (Variables|Default|GetClosestIntreractable))
  (:Started
    (if (Variables|Default|GetHasNearbyInteractable)
      (Utilities|IsValid _closestintreractable
        (:Is%20Valid
          (if (Utilities|DoesObjectImplementInterface _closestintreractable "/Script/Team24Project.Interactable")
            (Class|Interactable|Interact(Message) _closestintreractable)))))))

(event Input|EnhancedActionEvents|EnhancedInputActionIA_Jump
  (params (ActionValue :type Boolean) (ElapsedSeconds :type Float%20%28double-precision%29) (TriggeredSeconds :type Float%20%28double-precision%29) (InputAction :type Input%20Action%20Object%20Reference :default "/Game/Input/InputAssets/IA_Jump.IA_Jump"))
  (:Started
    (Default|OnJumpInput (Variables|Default|GetControlledCharacter))))

(event Input|EnhancedActionEvents|EnhancedInputActionIA_Move
  (params (ActionValue :type Vector%202D%20Structure) (ElapsedSeconds :type Float%20%28double-precision%29) (TriggeredSeconds :type Float%20%28double-precision%29) (InputAction :type Input%20Action%20Object%20Reference :default "/Game/Input/InputAssets/IA_Move.IA_Move"))
  (Default|OnMoveInput (Variables|Default|GetControlledCharacter) ActionValue))

(event Input|EnhancedActionEvents|EnhancedInputActionIA_Look
  (params (ActionValue :type Vector%202D%20Structure) (ElapsedSeconds :type Float%20%28double-precision%29) (TriggeredSeconds :type Float%20%28double-precision%29) (InputAction :type Input%20Action%20Object%20Reference :default "/Game/Input/InputAssets/IA_Look.IA_Look"))
  (Default|OnLookInput (Variables|Default|GetControlledCharacter) ActionValue))

(event EventBeginPlay
  (Development|PrintString "PC begin play")
  (if (Pawn|IsLocalController)
    (Development|PrintString "true")))

(event EventPossess
  (params (PossessedPawn :type Pawn%20Object%20Reference))
  (bind _asbp_player_character (Utilities|Casting|CastToBP_PlayerCharacter PossessedPawn)
    (:then
      (Variables|Default|SetControlledCharacter _asbp_player_character)
      (Development|PrintString "Pawn possessed")
      (Input|AddMappingContext (PlayerController|LocalPlayerSubsystems|GetEnhancedInputLocalPlayerSubsystem) "/Game/Input/InputAssets/IMC_DefaultInput.IMC_DefaultInput" 0 "(bIgnoreAllPressedKeysUntilRelease=True,bForceImmediately=False,bNotifyUserSettings=False)")
      (Development|PrintString "Input mapping context added"))
    (:CastFailed
      (Development|PrintString "Possess failed"))))

(fn ConstructionScript)

(fn AddNewInteractable
  (params (Actor :type Actor%20Object%20Reference%20%28by%20ref%29))
  (bind _returnvalue (Game|GetPlayerCharacter 0))
  (bind _returnvalue_2 (Transformation|GetActorLocation _returnvalue))
  (Utilities|IsValid (Variables|Default|GetClosestIntreractable)
    (:Is%20Valid
      (if (< (Math|Vector|Distance(Vector) (Transformation|GetActorLocation Actor) _returnvalue_2) (Math|Vector|Distance(Vector) _returnvalue_2 (Transformation|GetActorLocation (Variables|Default|GetClosestIntreractable))))
        (Variables|Default|SetClosestIntreractable Actor)
        (else
          (return))))
    (:Is%20Not%20Valid
      (Variables|Default|SetClosestIntreractable Actor)))
  (Variables|Default|SetHasNearbyInteractable true))

(fn RemoveInteractable
  (params (Actor :type Actor%20Object%20Reference%20%28by%20ref%29))
  (if (== Actor (Variables|Default|GetClosestIntreractable))
    (Variables|Default|SetHasNearbyInteractable (not (== Actor (Variables|Default|GetClosestIntreractable))))
    (Variables|Default|SetClosestIntreractable 0)))