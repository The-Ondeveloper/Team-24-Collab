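; Player controller for the AlexDM player character that handles input, the HUD and the pause menu.
; On possess it stores the character and adds the default Enhanced Input mapping context, then forwards move, look and jump input to that character.
; BeginPlay creates and initialises the HUD from the stored character.
; The pause input toggles game pause and the menu widget; left click is empty and right click only prints debug text.
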(event Input|EnhancedActionEvents|EnhancedInputActionIA_LeftClick
  (params (ActionValue :type Boolean) (ElapsedSeconds :type Float%20%28double-precision%29) (TriggeredSeconds :type Float%20%28double-precision%29) (InputAction :type Input%20Action%20Object%20Reference :default "/Game/Input/InputAssets/IA_LeftClick.IA_LeftClick")))

(event Input|EnhancedActionEvents|EnhancedInputActionIA_Jump
  (params (ActionValue :type Boolean) (ElapsedSeconds :type Float%20%28double-precision%29) (TriggeredSeconds :type Float%20%28double-precision%29) (InputAction :type Input%20Action%20Object%20Reference :default "/Game/Input/InputAssets/IA_Jump.IA_Jump"))
  (:Started
    (Default|OnJumpInput (Variables|Default|GetControlledCharacter))))

(event Input|EnhancedActionEvents|EnhancedInputActionIA_Move
  (params (ActionValue :type Vector%202D%20Structure) (ElapsedSeconds :type Float%20%28double-precision%29) (TriggeredSeconds :type Float%20%28double-precision%29) (InputAction :type Input%20Action%20Object%20Reference :default "/Game/Input/InputAssets/IA_Move.IA_Move"))
  (Default|OnMoveInput (Variables|Default|GetControlledCharacter) ActionValue))

(event Input|EnhancedActionEvents|EnhancedInputActionIA_Look
  (params (ActionValue :type Vector%202D%20Structure) (ElapsedSeconds :type Float%20%28double-precision%29) (TriggeredSeconds :type Float%20%28double-precision%29) (InputAction :type Input%20Action%20Object%20Reference :default "/Game/Input/InputAssets/IA_Look.IA_Look"))
  (Default|OnLookInput (Variables|Default|GetControlledCharacter) ActionValue))

(event Input|EnhancedActionEvents|EnhancedInputActionIA_RightClick
  (params (ActionValue :type Boolean) (ElapsedSeconds :type Float%20%28double-precision%29) (TriggeredSeconds :type Float%20%28double-precision%29) (InputAction :type Input%20Action%20Object%20Reference :default "/Game/Input/InputAssets/IA_RightClick.IA_RightClick"))
  (:Started
    (Development|PrintString "rclickpressed"))
  (:Completed
    (Development|PrintString "rclickreleased")))

(event Input|EnhancedActionEvents|EnhancedInputActionIA_Pause
  (params (ActionValue :type Boolean) (ElapsedSeconds :type Float%20%28double-precision%29) (TriggeredSeconds :type Float%20%28double-precision%29) (InputAction :type Input%20Action%20Object%20Reference :default "/Game/Input/InputAssets/IA_Pause.IA_Pause"))
  ;[0.15 0.15 0.15 0.5] Pause Input, Will Open Pause Menu and Can be Closed With the Input as well as the button in the pause menu
  (:Started
    (bind _output_get (Variables|Default|SetPaused? (not (Variables|Default|GetPaused?))))
    (Game|SetGamePaused _output_get)
    (if (Variables|Default|GetPaused?)
      (bind _returnvalue (UserInterface|CreateWidget "/Game/UI/WBP_PauseMenu.WBP_PauseMenu_C"))
      (bind _output_get_2 (Variables|Default|SetPauseWidget _returnvalue))
      (UserInterface|Viewport|AddtoViewport _output_get_2 0)
      (else
        (Widget|RemovefromParent _output_get_2)))))

(event Input|EnhancedActionEvents|EnhancedInputActionIA_AbilityPrimary
  (params (ActionValue :type Boolean) (ElapsedSeconds :type Float%20%28double-precision%29) (TriggeredSeconds :type Float%20%28double-precision%29) (InputAction :type Input%20Action%20Object%20Reference :default "/Game/Input/InputAssets/IA_AbilityPrimary.IA_AbilityPrimary")))

(event EventBeginPlay
  (bind _returnvalue (UserInterface|CreateWidget "/Game/UI/PlayerHUD/WBP_PlayerHUD.WBP_PlayerHUD_C"))
  (bind _output_get (Variables|Default|SetPlayerHUDWidget _returnvalue))
  (bind _asbp_alex_dmplayer_character (Utilities|Casting|CastToBP_AlexDMPlayerCharacter (Variables|Default|GetControlledCharacter)))
  (Default|InitialiseHUD _output_get _asbp_alex_dmplayer_character)
  (UserInterface|Viewport|AddtoPlayerScreen _output_get))

(event EventPossess
  (params (PossessedPawn :type Pawn%20Object%20Reference))
  (bind _asbp_player_character (Utilities|Casting|CastToBP_PlayerCharacter PossessedPawn))
  (Variables|Default|SetControlledCharacter _asbp_player_character)
  (Development|PrintString "Pawn possessed")
  (Input|AddMappingContext (PlayerController|LocalPlayerSubsystems|GetEnhancedInputLocalPlayerSubsystem) "/Game/Input/InputAssets/IMC_DefaultInput.IMC_DefaultInput" 0 "(bIgnoreAllPressedKeysUntilRelease=True,bForceImmediately=False,bNotifyUserSettings=False)")
  (Development|PrintString "Input mapping context added"))

(fn ConstructionScript)